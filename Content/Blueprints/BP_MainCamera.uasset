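; BP_MainCamera is a side-view follow camera that becomes the view target and tracks BP_Player.
; Each tick it copies the player camera component's X and Z, adding a height offset and holding Y at CamDistance.
; Events blend the view back to it, swap in a new player, or play a damage camera shake.
; Camposition stores a movement direction that this graph never reads.
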(event Custom|Camposition
  (params (Move :type Boolean))
  ;[0 1 0.5313] CamDirection
  (Variables|Default|SetDirection Move))

(event Custom|CameraShake
  ;[0.7344 0 1] CameraShake_Damage
  (Camera|PlayWorldCameraShake "/Game/Blueprints/BP_CameraShake_Damage.BP_CameraShake_Damage_C" (Transformation|GetActorLocation) 0.0 5e+02))

(event Custom|ActivateMainCam
  (Game|Player|SetViewTargetwithBlend (Game|GetPlayerController 0) self 2.0 "VTBlend_Linear" 0.0 false))

(event Custom|FindNewPlayer
  (params (Player :type BP%20Player%20Object%20Reference))
  ;[0 1 0.9766] ReconectingCam
  (Variables|Default|SetPlayer Player)
  (Game|Player|SetViewTargetwithBlend (Game|GetPlayerController 0) self 2.0 "VTBlend_Linear" 0.0 false))

(event EventBeginPlay
  ;[0 1 0.6719] INIT
  (Game|Player|SetViewTargetwithBlend (Game|GetPlayerController 0) self 0.0 "VTBlend_Linear" 0.0 false)
  (bind _asbp_player (Utilities|Casting|CastToBP_Player (Game|Player|GetPlayerPawn 0)))
  (bind _output_get (Variables|Default|SetPlayer _asbp_player))
  (Transformation|SetActorRelativeLocation (Math|Vector|MakeVector (.x (Transformation|GetActorLocation _output_get)) (Variables|Default|GetCamDistance) (+ (.z (Transformation|GetActorLocation _output_get)) (Variables|Default|GetAddingZPosition)))))

(event EventTick
  (params (DeltaSeconds :type Float%20%28single-precision%29))
  (bind _player (Variables|Default|GetPlayer))
  (bind _player_2 (Variables|Default|GetPlayer))
  (bind _camera (Variables|/Game/Blueprints/BP_Player.BP_Player_C|GetCamera _player))
  (bind _returnvalue (Transformation|GetWorldLocation _camera))
  ;[0 1 0.8828] Set Variables
  (Utilities|IsValid _player_2
    (:Is%20Valid
      (Variables|Default|SetPlayerXPosition (.x (Transformation|GetWorldLocation (Variables|/Game/Blueprints/BP_Player.BP_Player_C|GetCamera _player_2))))
      (Variables|Default|SetCameraXPositon (.x (Transformation|GetActorLocation)))
      (Transformation|SetActorLocation (Math|Vector|MakeVector (.x _returnvalue) (Variables|Default|GetCamDistance) (+ (.z _returnvalue) (Variables|Default|GetAddingZPosition))) false false))))

(fn ConstructionScript
  (bind _player (Variables|Default|GetPlayer))
  (bind _returnvalue (Transformation|GetActorLocation _player))
  (Utilities|IsValid _player
    (:Is%20Valid
      (Transformation|SetActorLocation (Math|Vector|MakeVector (.x _returnvalue) (Variables|Default|GetCameraLookForwardPosition) (.z _returnvalue)) false false))))