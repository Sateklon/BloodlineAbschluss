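; BP_Dornenbusch is a thorn bush hazard that damages the player pawn on entry and repeatedly while it moves inside.
; Begin and end overlap on CollisionComponent track whether player 0 is inside and apply the entry damage.
; Tick adds a fixed 0.1 per frame, independent of delta time, while X velocity is nonzero, resetting when it stops.
; When the timer reaches TimetoMakeDamage, MakeDamage resets it and applies Damage again.
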(event OnComponentBeginOverlap(CollisionComponent)
  (params (OverlappedComponent :type Primitive%20Component%20Object%20Reference) (OtherActor :type Actor%20Object%20Reference) (OtherComp :type Primitive%20Component%20Object%20Reference) (OtherBodyIndex :type Integer) (bFromSweep :type Boolean) (SweepResult :type Hit%20Result%20Structure%20%28by%20ref%29))
  (bind _returnvalue (Game|Player|GetPlayerPawn 0))
  (if (== OtherActor _returnvalue)
    (Variables|Default|SetisPlayerInside true)
    (bind _output_get (Variables|Default|SetPlayer _returnvalue))
    (Game|Damage|ApplyDamage _output_get (Variables|Default|GetDamage) 0 self)))

(event OnComponentEndOverlap(CollisionComponent)
  (params (OverlappedComponent :type Primitive%20Component%20Object%20Reference) (OtherActor :type Actor%20Object%20Reference) (OtherComp :type Primitive%20Component%20Object%20Reference) (OtherBodyIndex :type Integer))
  (if (== OtherActor (Game|Player|GetPlayerPawn 0))
    (Variables|Default|SetisPlayerInside false)))

(event Custom|MakeDamage
  ;[0 1 0.9531] Damage
  (Variables|Default|SetMoveTimer 0.0)
  (Game|Damage|ApplyDamage (Variables|Default|GetPlayer) (Variables|Default|GetDamage) 0 self))

(event EventBeginPlay)

(event EventTick
  (params (DeltaSeconds :type Float%20%28single-precision%29))
  ;[0.6875 1 0] Dornenlogik
  (if (Variables|Default|GetisPlayerInside)
    (if (not (Math|Float|NearlyEqual(Float) (.x (Transformation|GetVelocity (Variables|Default|GetPlayer))) 0.0 1e-06))
      (bind _output_get (Variables|Default|SetMoveTimer (+ (Variables|Default|GetMoveTimer) 0.1)))
      (if (>= _output_get (Variables|Default|GetTimetoMakeDamage))
        (CallFunction|MakeDamage))
      (else
        (Variables|Default|SetMoveTimer 0.0)))))

(fn ConstructionScript)