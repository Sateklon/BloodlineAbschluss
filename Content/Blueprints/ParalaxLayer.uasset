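; ParalaxLayer is an actor that acts as a parallax layer, shifting with a referenced camera.
; Each Tick, if the camera is valid, it sets its X and Z to the camera's position scaled by horizontal and vertical movement factors, minus a vertical offset on Z.
; Y stays at a hardcoded depth.
; BeginPlay stores the starting Z, but the movement does not use it.
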(event EventBeginPlay
  ;[0.875 1 0] Setup
  (Variables|Default|SetStartZ (.z (Transformation|GetActorLocation))))

(event EventTick
  (params (DeltaSeconds :type Float%20%28single-precision%29))
  (bind _camera (Variables|Default|GetCamera))
  (bind _returnvalue (Transformation|GetActorLocation _camera))
  ;[0 1 0.4375] Paralax
  (Utilities|IsValid _camera
    (:Is%20Valid
      (Transformation|SetActorLocation (Math|Vector|MakeVector (* (.x _returnvalue) (Variables|Default|GetHorizontalMovement)) -4e+02 (- (* (.z _returnvalue) (Variables|Default|GetVerticalMovement)) (Variables|Default|GetVerticalOptimasation))) false false))))

(fn ConstructionScript)