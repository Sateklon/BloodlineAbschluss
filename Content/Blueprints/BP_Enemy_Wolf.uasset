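; BP_Enemy_Wolf is a wolf enemy Blueprint that adds a lunging charge attack to its parent class.
; WolfAttackCharge launches the character slightly upward, waits briefly, then launches it along world X in the direction it faces, chosen by the sign of its forward vector.
; Tick passes through to the parent, and the construction script only runs the parent's version.
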(event Custom|WolfAttackCharge
  (Character|LaunchCharacter (Math|Vector|MakeVector 0.0 0.0 1e+02) false false)
  (Utilities|FlowControl|Delay 0.05)
  (Character|LaunchCharacter (Math|Vector|MakeVector (Math|Interpolation|Ease "Linear" 1.0 0.0 (Math|Float|SelectFloat 5e+02 -5e+02 (>= (.x (Transformation|GetActorForwardVector)) 0.0))) 0.0 0.0) false false))

(event EventBeginPlay
  (|CallParentFunction) ; This node is disabled and will not be called.\nDrag off pins to build functionality.
)

(event Collision|EventActorBeginOverlap
  (params (OtherActor :type Actor%20Object%20Reference)))

(event EventTick
  (params (DeltaSeconds :type Float%20%28single-precision%29))
  (|CallParentFunction DeltaSeconds))

(fn ConstructionScript
  (|CallParentFunction))