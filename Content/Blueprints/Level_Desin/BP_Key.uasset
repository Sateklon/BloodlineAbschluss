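; BP_Key is a key pickup that counts toward opening a linked gate when the player collects it.
; Overlapping its sphere with the player pawn runs Collect and plays a 2D key sound.
; Collect casts DoorToKey to BP_GateKlein or BP_GateGroß, calls PlayerCollectKey, then destroys the key, which stays if no valid door is linked.
; GameMode is cached on BeginPlay, but its collectable-message logic is disconnected.
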(event OnComponentBeginOverlap(Sphere)
  (params (OverlappedComponent :type Primitive%20Component%20Object%20Reference) (OtherActor :type Actor%20Object%20Reference) (OtherComp :type Primitive%20Component%20Object%20Reference) (OtherBodyIndex :type Integer) (bFromSweep :type Boolean) (SweepResult :type Hit%20Result%20Structure%20%28by%20ref%29))
  (bind _returnvalue (Game|Player|GetPlayerPawn 0))
  ;[1 0 0.6094] Overlapping with Player
  (if (== OtherActor _returnvalue)
    (CallFunction|Collect _returnvalue)
    ;;[0 1 0.0625] Sound
    (Class|FMODBlueprintStatics|PlayEvent2D "/Game/FMOD/Events/KeysCollect_object-metal-keys-handling-02.KeysCollect_object-metal-keys-handling-02")))

(event EventBeginPlay
  (bind _asgm_plattformer (Utilities|Casting|CastToGM_Plattformer (Game|GetGameMode)))
  (Variables|Default|SetGameMode _asgm_plattformer))

(event EventCollect
  (params (Collector :type Pawn%20Object%20Reference))
  ;[0.2656 0 1] CollectKey
  (bind _doortokey (Variables|Default|GetDoorToKey)
    (:then
      (bind _asbp_gate_klein (Utilities|Casting|CastToBP_GateKlein _doortokey)
        (:then
          (Default|PlayerCollectKey _asbp_gate_klein)
          (Actor|DestroyActor :!label _label))
        (:CastFailed
          (bind _doortokey_2 (Variables|Default|GetDoorToKey)
            (:then
              (bind _asbp_gate_groß (Utilities|Casting|CastToBP_GateGroß _doortokey_2)
                (:then
                  (Default|PlayerCollectKey _asbp_gate_groß)
                  (goto _label))
                (:CastFailed
                  (Actor|DestroyActor))))
            (:else)))))
    (:else)))

(fn ConstructionScript)