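; Checkpoint actor for the platformer that, on player overlap, fully heals the player and moves the respawn point here.
; It passes the Arrow's transform, minus Y location, and a camera spline to GM_Plattformer, then refills potions and respawns actors through it.
; Activation sounds play only once, while three point lights flicker continuously via ping-ponging timelines.
; The logic adding it to the reached-checkpoints list is disconnected.
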(event Custom|Licht2Anim
  ;[1 0.375 0] Comment
  (Utilities|FlowControl|FlipFlop
    (:A
      (bind _alpha (Timeline|Timeline PlayFromStart)
        (:Update
          (Rendering|Components|Light|SetIntensity (Variables|Default|GetPointLight2) (Math|Float|Lerp 1e+04 2e+04 _alpha)))
        (:Finished
          (CallFunction|Licht2Anim))))
    (:B
      (Timeline|Timeline ReverseFromEnd))))

(event Custom|Licht1Anim
  ;[0 0.2734 1] Comment
  (Utilities|FlowControl|FlipFlop
    (:A
      (bind _alpha (Timeline|Lichtflakern PlayFromStart)
        (:Update
          (Rendering|Components|Light|SetIntensity (Variables|Default|GetPointLight1) (Math|Float|Lerp 1e+04 2e+04 _alpha)))
        (:Finished
          (CallFunction|Licht1Anim))))
    (:B
      (Timeline|Lichtflakern ReverseFromEnd))))

(event Custom|Licht3Anim
  ;[1 0.5625 0] Comment
  (Utilities|FlowControl|FlipFlop
    (:A
      (bind _alpha (Timeline|Timeline_0 PlayFromStart)
        (:Update
          (Rendering|Components|Light|SetIntensity (Variables|Default|GetPointLight3) (Math|Float|Lerp 1e+04 2e+04 _alpha)))
        (:Finished
          (CallFunction|Licht3Anim))))
    (:B
      (Timeline|Timeline_0 ReverseFromEnd))))

(event EventBeginPlay
  (bind _asgm_plattformer (Utilities|Casting|CastToGM_Plattformer (Game|GetGameMode)))
  (Variables|Default|SetGamMode _asgm_plattformer)
  (CallFunction|Licht1Anim)
  (CallFunction|Licht2Anim)
  (CallFunction|Licht3Anim))

(event Collision|EventActorBeginOverlap
  (params (OtherActor :type Actor%20Object%20Reference))
  (bind _arrow (Variables|Default|GetArrow))
  (bind _returnvalue (Transformation|GetWorldTransform _arrow))
  ;[1 0 0.6797] Wenn der Spieler in TriggerBox läuft
  (bind _asbp_player (Utilities|Casting|CastToBP_Player OtherActor))
  ;[0.6406 1 0] Heile den Spieler voll
  (Default|Fulheal _asbp_player)
  ;[1 0 0.4453] Setze den Spieler Spawnpoint
  (bind _asgm_plattformer (Utilities|Casting|CastToGM_Plattformer (Game|GetGameMode)))
  (Variables|/Game/Blueprints/GM_Plattformer.GM_Plattformer_C|SetPlayer%20Spawnpoint _asgm_plattformer (Math|Transform|MakeTransform (Math|Vector|MakeVector (.x (.location _returnvalue)) 0.0 (.z (.location _returnvalue))) (.rotation _returnvalue) (.scale _returnvalue)))
  (Default|RespawningSpline _asgm_plattformer (Variables|Default|GetRespawnCameraSpline))
  ;[1 0.4219 0] Spiel die Checkpoint aktivierungs-Anim
  (Variables|Default|SetActive true)
  (Utilities|FlowControl|Sequence
    (:then_0
      ;[0.1719 1 0] Potion Refill
      (bind _asgm_plattformer_2 (Utilities|Casting|CastToGM_Plattformer (Game|GetGameMode)))
      (Default|UpdateUseablePotions _asgm_plattformer_2)
      ;[1 0.3516 0] Respawn Dinge
      (Default|RespwaningActors _asgm_plattformer_2))
    (:then_1
      (Utilities|FlowControl|DoOnce false
        (:Completed
          (Class|FMODBlueprintStatics|PlayEvent2D "/Game/FMOD/Events/Checkpoint01_ES_Impact_Designed_1_-_SFX_Producer.Checkpoint01_ES_Impact_Designed_1_-_SFX_Producer")
          (Class|FMODBlueprintStatics|PlayEventatLocation "/Game/FMOD/Events/CheckpointActivatedSurkling__Into_Water.CheckpointActivatedSurkling__Into_Water" (Transformation|GetActorTransform)))))))

(fn ConstructionScript)