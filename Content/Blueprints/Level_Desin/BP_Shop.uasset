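; BP_Shop is an interactable shop actor for the platformer that registers its items in the game mode's AllShopItems list on BeginPlay.
; Box overlap shows a sprite prompt and flags the player as able to interact until exit.
; Interact pushes WBP_Shop onto the HUD's gameplay stack and permanently blocks further prompts.
; ShopClosed marks it closed and, once only, records the shop in the GameInstance's ListOfShops for saving.
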(event OnComponentBeginOverlap(Box)
  (params (OverlappedComponent :type Primitive%20Component%20Object%20Reference) (OtherActor :type Actor%20Object%20Reference) (OtherComp :type Primitive%20Component%20Object%20Reference) (OtherBodyIndex :type Integer) (bFromSweep :type Boolean) (SweepResult :type Hit%20Result%20Structure%20%28by%20ref%29))
  ;[0 0.2031 1] Interact ?
  (if (not (Variables|Default|GetPlayer%20Has%20Interacted))
    (bind _asbp_player (Utilities|Casting|CastToBP_Player OtherActor))
    (Default|PlayerCanInteract _asbp_player self)
    (Rendering|SetVisibility (Variables|Default|GetPaperSprite) true false)))

(event OnComponentEndOverlap(Box)
  (params (OverlappedComponent :type Primitive%20Component%20Object%20Reference) (OtherActor :type Actor%20Object%20Reference) (OtherComp :type Primitive%20Component%20Object%20Reference) (OtherBodyIndex :type Integer))
  ;[0 1 0.1797] End Overlap
  (bind _asbp_player (Utilities|Casting|CastToBP_Player OtherActor))
  (Default|PlayerCannotInteract _asbp_player)
  (Rendering|SetVisibility (Variables|Default|GetPaperSprite) false false))

(event Custom|ShopClosed
  (bind _self self)
  ;[0.9688 1 0] Shop Closed
  (Variables|Default|SetisShopclosed true)
  (Utilities|FlowControl|DoOnce false
    (:Completed
      ;[0.3828 1 0] Save System
      (bind _settings (Class|BPIGameInstance|GetSettings(Message) (Game|GetGameInstance)))
      (Utilities|Array|RemoveItem (Variables|/Game/Blueprints/SaveSystem/BP_SettingsSave.BP_SettingsSave_C|GetListOfShops _settings) _self)
      (Utilities|Array|Add (Variables|/Game/Blueprints/SaveSystem/BP_SettingsSave.BP_SettingsSave_C|GetListOfShops _settings) _self))))

(event EventBeginPlay
  (|CallParentFunction)
  ;[0.8281 0 1] get Game Manager
  (bind _asgm_plattformer (Utilities|Casting|CastToGM_Plattformer (Game|GetGameMode)))
  (bind _output_get (Variables|Default|SetGameManager _asgm_plattformer))
  ;[0 0.7891 1] Füge die ShopItems zu den "All Shop Items" hinzu
  (for _array_element (Variables|Default|GetShopItems)
    (Utilities|Array|RemoveItem (Variables|/Game/Blueprints/GM_Plattformer.GM_Plattformer_C|GetAllShopItems _output_get) _array_element)
    (Utilities|Array|Add (Variables|/Game/Blueprints/GM_Plattformer.GM_Plattformer_C|GetAllShopItems _output_get) _array_element)))

(event Collision|EventActorBeginOverlap
  (params (OtherActor :type Actor%20Object%20Reference))
  (|CallParentFunction OtherActor) ; This node is disabled and will not be called.\nDrag off pins to build functionality.
)

(event EventInteract
  ;[1 0.5859 0] Öffne den Shop
  (Variables|Default|SetPlayer%20Has%20Interacted true)
  (Variables|Default|SetisShopclosed false)
  (Class|BPIHUD|PushtoGameplayStack(Message) (HUD|GetHUD (Game|GetPlayerController 0)) "/Game/Blueprints/UI/WBP_Shop.WBP_Shop_C"))

(fn ConstructionScript
  (|CallParentFunction))