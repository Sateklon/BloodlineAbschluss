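; BP_GateGroß is a large gate the player opens by interacting, optionally requiring a key granted through PlayerCollectKey.
; Two triggers show a prompt sprite and register it with BP_Player, with FalseTrigger marking the wrong side, where interaction only wobbles.
; DoOnce-guarded Open and Wobble flags start each reaction, with rumble and sound on opening.
; OpenDoorOver disables collision, WobblingOver re-arms interaction, and the GameMode save code is disconnected.
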(event OnComponentBeginOverlap(DoorInteractionTrigger)
  (params (OverlappedComponent :type Primitive%20Component%20Object%20Reference) (OtherActor :type Actor%20Object%20Reference) (OtherComp :type Primitive%20Component%20Object%20Reference) (OtherBodyIndex :type Integer) (bFromSweep :type Boolean) (SweepResult :type Hit%20Result%20Structure%20%28by%20ref%29))
  ;[1 0.2109 0] Player Can Interact
  (if (not (Variables|Default|GetPlayerhas%20Interacted))
    (if (not (Variables|Default|GetisOpen))
      (bind _asbp_player (Utilities|Casting|CastToBP_Player OtherActor))
      (Default|PlayerCanInteract _asbp_player self)
      (Rendering|SetVisibility (Variables|Default|GetPaperSprite) true false))))

(event OnComponentEndOverlap(DoorInteractionTrigger)
  (params (OverlappedComponent :type Primitive%20Component%20Object%20Reference) (OtherActor :type Actor%20Object%20Reference) (OtherComp :type Primitive%20Component%20Object%20Reference) (OtherBodyIndex :type Integer))
  ;[0 0.1562 1] Player Cannot Interact
  (bind _asbp_player (Utilities|Casting|CastToBP_Player OtherActor))
  (Default|PlayerCannotInteract _asbp_player)
  (Rendering|SetVisibility (Variables|Default|GetPaperSprite) false false))

(event OnComponentBeginOverlap(FalseTrigger)
  (params (OverlappedComponent :type Primitive%20Component%20Object%20Reference) (OtherActor :type Actor%20Object%20Reference) (OtherComp :type Primitive%20Component%20Object%20Reference) (OtherBodyIndex :type Integer) (bFromSweep :type Boolean) (SweepResult :type Hit%20Result%20Structure%20%28by%20ref%29))
  ;[1 0.2109 0] Player Can Interact (falsche Seite) oder später mit Schlüssel, was gecodet werden muss
  (if (not (Variables|Default|GetisOpen))
    (bind _asbp_player (Utilities|Casting|CastToBP_Player OtherActor))
    (Default|PlayerCanInteract _asbp_player self)
    (Rendering|SetVisibility (Variables|Default|GetPaperSprite) true false)
    (Variables|Default|Setwobbling true)))

(event OnComponentEndOverlap(FalseTrigger)
  (params (OverlappedComponent :type Primitive%20Component%20Object%20Reference) (OtherActor :type Actor%20Object%20Reference) (OtherComp :type Primitive%20Component%20Object%20Reference) (OtherBodyIndex :type Integer))
  ;[1 0.8672 0] Player cant Interact
  (bind _asbp_player (Utilities|Casting|CastToBP_Player OtherActor))
  (Default|PlayerCannotInteract _asbp_player)
  (Rendering|SetVisibility (Variables|Default|GetPaperSprite) false false)
  (Variables|Default|Setwobbling false))

(event Custom|PlayerCollectKey
  ;[1 0 0.8906] Player found Key
  (Variables|Default|SetInteractable true))

(event Custom|WobblingOver
  ;[1 0.1406 0] Interaction
  (Utilities|FlowControl|Sequence
    (:then_0
      (Utilities|FlowControl|DoOnce false) ; enters at Reset
    )
    (:then_1
      ;;[0 1 0.8125] Player hat noch nicht den key
      (Variables|Default|SetPlayerhas%20Interacted false)
      (Variables|Default|SetWobble false)
      (Utilities|FlowControl|DoOnce false) ; enters at Reset
    )))

(event Custom|OpenDoorOver
  ;[1 0.1406 0] Interaction
  ;;[0 1 0.2969] Player hat den Key
  (Utilities|FlowControl|Sequence
    (:then_0
      (Variables|Default|SetOpen false)
      (Utilities|FlowControl|DoOnce false) ; enters at Reset
    )
    (:then_1
      ;;[0.05469 0 1] Stop die vibration
      (Game|Feedback|ClientStopForceFeedback (Game|GetPlayerController 0) "/Game/Blueprints/ControllerVibration/DoorOpen.DoorOpen" "None")
      ;;[1 0.9141 0] Mach Collision aus
      (Collision|SetCollisionEnabled (Variables|Default|GetDoorCollision) "NoCollision")
      ;;[1 0.7734 0] Ist Offen
      (Variables|Default|SetisOpen true))))

(event EventBeginPlay
  (bind _asgm_plattformer (Utilities|Casting|CastToGM_Plattformer (Game|GetGameMode)))
  (Variables|Default|SetGameMode _asgm_plattformer))

(event EventInteract
  ;[1 0.1406 0] Interaction
  (if (and (not (Variables|Default|GetisOpen)) (not (Variables|Default|GetPlayerhas%20Interacted)))
    (if (not (Variables|Default|Getwobbling))
      (Variables|Default|SetPlayerhas%20Interacted true)
      (if (or (not (Variables|Default|GetDoor%20Need%20Key)) (Variables|Default|GetInteractable))
        ;;[0 1 0.2969] Player hat den Key
        (Rendering|SetVisibility (Variables|Default|GetPaperSprite) false false)
        (Variables|Default|SetInteractable false)
        (Utilities|FlowControl|DoOnce false
          (:Completed
            (Variables|Default|SetOpen true)
            (Game|Feedback|ClientPlayForceFeedback (Game|GetPlayerController 0) "/Game/Blueprints/ControllerVibration/DoorOpen.DoorOpen" "None" false false false)
            ;;[0.1484 0 1] Sound
            (Class|FMODBlueprintStatics|PlayEvent2D "/Game/FMOD/Events/DoorOpening01_Shipping_Container__Drag__Creak__Squeak__Heavy__Deep__Big_Reverb_06.DoorOpening01_Shipping_Container__Drag__Creak__Squeak__Heavy__Deep__Big_Reverb_06")))
        (else
          ;;[0 1 0.8125] Player hat noch nicht den key
          (Rendering|SetVisibility (Variables|Default|GetPaperSprite) false false)
          (Utilities|FlowControl|Delay 1.0)
          (Variables|Default|SetPlayerhas%20Interacted false)
          (Utilities|FlowControl|DoOnce false
            (:Completed
              (Variables|Default|SetWobble true)))))
      (else
        (Utilities|FlowControl|DoOnce false
          (:Completed
            (Variables|Default|SetWobble true)
            (Variables|Default|SetPlayerhas%20Interacted true)))))))

(fn ConstructionScript)