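; BP_SpecialStone is a collectible stone pickup in a platformer, collected when BP_Player overlaps its sphere.
; Collection reports the stone type to GM_Plattformer, triggers its Steam achievement call and shows info text in the gameplay widget.
; The actor then destroys itself, and a collect sound plays.
; A looping timeline wobble that offsets its height is defined, but its call is disconnected.
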(event OnComponentBeginOverlap(Sphere)
  (params (OverlappedComponent :type Primitive%20Component%20Object%20Reference) (OtherActor :type Actor%20Object%20Reference) (OtherComp :type Primitive%20Component%20Object%20Reference) (OtherBodyIndex :type Integer) (bFromSweep :type Boolean) (SweepResult :type Hit%20Result%20Structure%20%28by%20ref%29))
  ;[1 0.2812 0] overlap
  (bind _asbp_player (Utilities|Casting|CastToBP_Player OtherActor))
  (if true
    (CallFunction|Collect _asbp_player)
    ;;[0.8516 1 0] Sound
    (Class|FMODBlueprintStatics|PlayEvent2D "/Game/FMOD/Events/Collect02_Cutlery__Hit_Dish.Collect02_Cutlery__Hit_Dish")))

(event Custom|WobbleAnimation
  (bind _returnvalue (Transformation|GetActorLocation))
  ;[1 0.4219 0] ANIM
  (bind _alpha (Timeline|Timeline Play)
    (:Update
      (Transformation|SetActorLocation (Math|Vector|MakeVector (.x _returnvalue) (.y _returnvalue) (+ (.z _returnvalue) _alpha)) false false))
    (:Finished
      (CallFunction|RestartAnim))))

(event Custom|RestartAnim
  (bind _returnvalue (Transformation|GetActorLocation))
  ;[1 0.4219 0] ANIM
  (bind _alpha (Timeline|Timeline PlayFromStart)
    (:Update
      (Transformation|SetActorLocation (Math|Vector|MakeVector (.x _returnvalue) (.y _returnvalue) (+ (.z _returnvalue) _alpha)) false false))
    (:Finished
      (CallFunction|RestartAnim))))

(event EventBeginPlay
  (bind _asgm_plattformer (Utilities|Casting|CastToGM_Plattformer (Game|GetGameMode)))
  (Variables|Default|SetGameMode _asgm_plattformer))

(event EventCollect
  (params (Collector :type Pawn%20Object%20Reference))
  (bind _gamemode (Variables|Default|GetGameMode))
  (bind _wbp_main (Variables|/Game/Blueprints/GM_Plattformer.GM_Plattformer_C|GetWBP_Main _gamemode))
  (bind _wbp_gameplay (Variables|/Game/Blueprints/UI/WBP_Main.WBP_Main_C|GetWBP_Gameplay _wbp_main))
  (bind _infotext (Variables|/Game/Blueprints/UI/WBP_Gameplay.WBP_Gameplay_C|GetInfotext _wbp_gameplay))
  ;[0 0.2266 1] Collect
  (Default|CollectSpecialStone (Variables|Default|GetGameMode) (Variables|Default|GetStonetype))
  ;;[0 0.6953 1] SteamAchievment
  (Default|SASpecialStoneCollect (Variables|Default|GetGameMode))
  (Default|SetupInfotext _infotext (Variables|Default|GetInfotext))
  (Widget|SetVisibility _infotext "Visible")
  (Actor|DestroyActor))

(fn ConstructionScript)