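; A bat (Fledermaus) level actor that reacts to the player's approach and flies away.
; Two trigger overlaps set idle and fly flags, with fly locking out idle changes.
; The Startflying event, not called within this file, runs once: the bat drops while squeaking, then climbs away and is destroyed after a delay.
; Tick moves it by fixed per-frame world offsets, so speed depends on frame rate.
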(event OnComponentBeginOverlap(IdleTrigger)
  (params (OverlappedComponent :type Primitive%20Component%20Object%20Reference) (OtherActor :type Actor%20Object%20Reference) (OtherComp :type Primitive%20Component%20Object%20Reference) (OtherBodyIndex :type Integer) (bFromSweep :type Boolean) (SweepResult :type Hit%20Result%20Structure%20%28by%20ref%29))
  ;[1 0.9375 0] IdleTrigger
  (if (== OtherActor (Game|Player|GetPlayerPawn 0))
    (if (not (Variables|Default|GetTriggerFly))
      (Variables|Default|SetTriggerIdle true))))

(event OnComponentEndOverlap(IdleTrigger)
  (params (OverlappedComponent :type Primitive%20Component%20Object%20Reference) (OtherActor :type Actor%20Object%20Reference) (OtherComp :type Primitive%20Component%20Object%20Reference) (OtherBodyIndex :type Integer))
  ;[0 1 0.4609] IdleExitTrigger
  (if (== OtherActor (Game|Player|GetPlayerPawn 0))
    (if (not (Variables|Default|GetTriggerFly))
      (Variables|Default|SetTriggerIdle false))))

(event OnComponentBeginOverlap(FlyTrigger)
  (params (OverlappedComponent :type Primitive%20Component%20Object%20Reference) (OtherActor :type Actor%20Object%20Reference) (OtherComp :type Primitive%20Component%20Object%20Reference) (OtherBodyIndex :type Integer) (bFromSweep :type Boolean) (SweepResult :type Hit%20Result%20Structure%20%28by%20ref%29))
  ;[0 0.6719 1] FlyTrigger
  (if (== OtherActor (Game|Player|GetPlayerPawn 0))
    (Variables|Default|SetTriggerFly true)))

(event Custom|Startflying
  (Utilities|FlowControl|DoOnce false
    (:Completed
      (Variables|Default|SetFalling true)
      (Class|FMODBlueprintStatics|PlayEvent2D "/Game/FMOD/Events/BatQuiek.BatQuiek")
      (Utilities|FlowControl|Delay 1.0)
      (Class|FMODBlueprintStatics|PlayEvent2D "/Game/FMOD/Events/BatQuiek.BatQuiek")
      (Variables|Default|SetFalling false)
      (Variables|Default|SetStartFly true)
      (Utilities|FlowControl|Delay 2e+01)
      (Actor|DestroyActor))))

(event EventBeginPlay)

(event Collision|EventActorBeginOverlap
  (params (OtherActor :type Actor%20Object%20Reference)))

(event EventTick
  (params (DeltaSeconds :type Float%20%28single-precision%29))
  (bind _returnvalue (Transformation|GetActorLocation))
  (bind _returnvalue_2 (Transformation|GetActorLocation))
  (Utilities|FlowControl|Sequence
    (:then_0
      (if (Variables|Default|GetFalling)
        (Transformation|SetActorLocation (Math|Vector|MakeVector (.x _returnvalue) (.y _returnvalue) (- (.z _returnvalue) 5.0)) false false)))
    (:then_1
      (if (Variables|Default|GetStartFly)
        (Transformation|SetActorLocation (Math|Vector|MakeVector (- (.x _returnvalue_2) 5.0) (.y _returnvalue_2) (+ (.z _returnvalue_2) 3.0)) false false)))))

(fn ConstructionScript)