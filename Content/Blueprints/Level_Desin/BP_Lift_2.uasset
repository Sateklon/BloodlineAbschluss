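; BP_Lift_2 is a three-level lift that moves its platform vertically when the player interacts.
; Its up and down trigger boxes, or external levers via LevelRequest, pick a target level through LevelOrder and register the lift as the player's interactable.
; Interact plays a timeline that lerps the platform's relative Z to that level's marker, updating the current level when finished.
; New orders and interactions are ignored while it moves.
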(event OnComponentBeginOverlap(InteractionBoxUP)
  (params (OverlappedComponent :type Primitive%20Component%20Object%20Reference) (OtherActor :type Actor%20Object%20Reference) (OtherComp :type Primitive%20Component%20Object%20Reference) (OtherBodyIndex :type Integer) (bFromSweep :type Boolean) (SweepResult :type Hit%20Result%20Structure%20%28by%20ref%29))
  (bind _currentliftlevel (Variables|Default|GetCurrentLiftLevel))
  ;[1 0 0.5859] Interaction vom Lift Selbst
  ;;[1 0 0.75] Nach oben
  (bind _asbp_player (Utilities|Casting|CastToBP_Player OtherActor))
  (if (not (Variables|Default|GetisMoving))
    (if (< _currentliftlevel 2)
      (CallFunction|LevelOrder (+ _currentliftlevel 1))
      (Default|PlayerCanInteract _asbp_player self)
      (else
        (Default|PlayerCannotInteract _asbp_player)))))

(event OnComponentEndOverlap(InteractionBoxUP)
  (params (OverlappedComponent :type Primitive%20Component%20Object%20Reference) (OtherActor :type Actor%20Object%20Reference) (OtherComp :type Primitive%20Component%20Object%20Reference) (OtherBodyIndex :type Integer))
  ;[1 0 0.5859] Interaction vom Lift Selbst
  ;;[1 0 0.75] Nach oben
  (bind _asbp_player (Utilities|Casting|CastToBP_Player OtherActor))
  (Default|PlayerCannotInteract _asbp_player))

(event OnComponentBeginOverlap(InteractionBoxDOWN)
  (params (OverlappedComponent :type Primitive%20Component%20Object%20Reference) (OtherActor :type Actor%20Object%20Reference) (OtherComp :type Primitive%20Component%20Object%20Reference) (OtherBodyIndex :type Integer) (bFromSweep :type Boolean) (SweepResult :type Hit%20Result%20Structure%20%28by%20ref%29))
  (bind _currentliftlevel (Variables|Default|GetCurrentLiftLevel))
  ;[1 0 0.5859] Interaction vom Lift Selbst
  ;;[0 0.3437 1] Nach unten
  (bind _asbp_player (Utilities|Casting|CastToBP_Player OtherActor))
  (if (not (Variables|Default|GetisMoving))
    (if (> _currentliftlevel 0)
      (CallFunction|LevelOrder (- _currentliftlevel 1))
      (Default|PlayerCanInteract _asbp_player self)
      (else
        (Default|PlayerCannotInteract _asbp_player)))))

(event OnComponentEndOverlap(InteractionBoxDOWN)
  (params (OverlappedComponent :type Primitive%20Component%20Object%20Reference) (OtherActor :type Actor%20Object%20Reference) (OtherComp :type Primitive%20Component%20Object%20Reference) (OtherBodyIndex :type Integer))
  ;[1 0 0.5859] Interaction vom Lift Selbst
  ;;[0 0.3437 1] Nach unten
  (bind _asbp_player (Utilities|Casting|CastToBP_Player OtherActor))
  (Default|PlayerCannotInteract _asbp_player))

(event Custom|LevelRequest
  (params (Level :type Integer))
  ;[0.9922 0 1] LevelRequest (von den anderen Hebeln)
  (if (and (!= Level (Variables|Default|GetCurrentLiftLevel)) (not (Variables|Default|GetisMoving)))
    (Variables|Default|SetRequested%20Level Level)
    (bind _asbp_player (Utilities|Casting|CastToBP_Player (Game|Player|GetPlayerPawn 0)))
    (Default|PlayerCanInteract _asbp_player self)
    (CallFunction|LevelOrder (Variables|Default|GetRequested%20Level))
    (else
      (bind _asbp_player_2 (Utilities|Casting|CastToBP_Player (Game|Player|GetPlayerPawn 0)))
      (Default|PlayerCannotInteract _asbp_player_2))))

(event Custom|LevelOrder
  (params (Ordering%20Level :type Integer))
  ;[1 0.7734 0] Level Order
  (if (not (Variables|Default|GetisMoving))
    (switch int Ordering%20Level
      (:0
        (Variables|Default|SetRequested%20Level 0)
        (Variables|Default|SetTargetZValue (.z (Variables|/Script/Engine.SceneComponent|GetRelativeLocation (Variables|Default|GetLevel%20-1%20%280%29)))))
      (:1
        (Variables|Default|SetRequested%20Level 1)
        (Variables|Default|SetTargetZValue (.z (Variables|/Script/Engine.SceneComponent|GetRelativeLocation (Variables|Default|GetLevel%200%20%281%29)))))
      (:2
        (Variables|Default|SetRequested%20Level 2)
        (Variables|Default|SetTargetZValue (.z (Variables|/Script/Engine.SceneComponent|GetRelativeLocation (Variables|Default|GetLevel%201%20%282%29))))))))

(event EventBeginPlay)

(event EventInteract
  ;[0 0.1094 1] LiftInteract
  ;;[1 0.2578 0] Lift oder Hebel nur Interagierbar, solang der Lift in Ruhelage ist
  (if (not (Variables|Default|GetisMoving))
    ;;[0.1719 1 0] LiftMovement
    (bind _alpha (Timeline|BesseresLiftMovement PlayFromStart)
      (:Update
        (Variables|Default|SetisMoving true)
        (Transformation|SetRelativeLocation (Variables|Default|GetPlattform) (Math|Vector|MakeVector 0.0 0.0 (Math|Float|Lerp (Variables|Default|GetCurrentZValue) (Variables|Default|GetTargetZValue) _alpha)) false false))
      (:Finished
        (Variables|Default|SetisMoving false)
        (Variables|Default|SetCurrentZValue (.z (Variables|/Script/Engine.SceneComponent|GetRelativeLocation (Variables|Default|GetPlattform))))
        (Variables|Default|SetCurrentLiftLevel (Variables|Default|GetRequested%20Level))))))

(fn ConstructionScript)