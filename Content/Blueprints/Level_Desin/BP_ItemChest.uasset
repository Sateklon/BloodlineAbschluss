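; BP_ItemChest is an interactable chest for the platformer that presents an item to the player.
; BeginPlay caches the platformer game mode and player pawn.
; Interact flags the chest as used and hides its sprite, then a DoOnce plays a creak sound and has the game mode show the item message.
; GetConditions returns a fixed condition and item type; the node recording opened chests in the game mode is unconnected.
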(event EventBeginPlay
  (|CallParentFunction)
  (bind _asgm_plattformer (Utilities|Casting|CastToGM_Plattformer (Game|GetGameMode)))
  (Variables|Default|SetGameMode _asgm_plattformer)
  (bind _asbp_player (Utilities|Casting|CastToBP_Player (Game|Player|GetPlayerPawn 0)))
  (Variables|Default|SetBP_Player _asbp_player))

(event EventInteract
  ;[0 1 0.6953] Spieler intteragiert
  (Variables|Default|SetPlayerHasInteracted true)
  (Rendering|SetVisibility (Variables|Default|GetPaperSprite) false false)
  (Utilities|FlowControl|DoOnce false
    (:Completed
      ;[0.4062 1 0] Sound
      (Class|FMODBlueprintStatics|PlayEvent2D "/Game/FMOD/Events/Chest_Open_Open__Creak_02.Chest_Open_Open__Creak_02")
      ;[0 0.1094 1] Show Message
      (Default|ShowMessage (Variables|Default|GetGameMode) (Variables|Default|GetItem)))))

(fn ConstructionScript
  (|CallParentFunction))

(fn GetConditions
  (return "NewEnumerator3" "NewEnumerator0"))