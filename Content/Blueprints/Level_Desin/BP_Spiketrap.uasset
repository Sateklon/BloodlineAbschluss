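; BP_Spiketrap is a level trap that cycles spikes and damages the player.
; Once the player first enters Triggerrange, Tick runs a DoOnce-gated delay loop that toggles Release on timings scaled by Looptime, with no stop condition.
; A separate Damage event, not called within this graph, applies SpikeDamage to the player overlapping SpikeDamageBox, using a second DoOnce reset after a short delay to limit repeat hits.
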(event OnComponentBeginOverlap(Triggerrange)
  (params (OverlappedComponent :type Primitive%20Component%20Object%20Reference) (OtherActor :type Actor%20Object%20Reference) (OtherComp :type Primitive%20Component%20Object%20Reference) (OtherBodyIndex :type Integer) (bFromSweep :type Boolean) (SweepResult :type Hit%20Result%20Structure%20%28by%20ref%29))
  ;[1 0.7031 0] Ist der Player in Range (Start des Loops)
  (if (== OtherActor (Game|Player|GetPlayerPawn 0))
    (Variables|Default|SetisPlayerInRange true)))

(event Custom|Damage
  (for _array_element (Collision|GetOverlappingActors (Variables|Default|GetSpikeDamageBox) "/Script/Engine.Actor" :!class /Script/Engine.PrimitiveComponent)
    (if (== _array_element (Game|Player|GetPlayerPawn 0))
      (Utilities|FlowControl|DoOnce false
        (:Completed
          (Game|Damage|ApplyDamage _array_element (Variables|Default|GetSpikeDamage) 0 self)))))
  (Utilities|FlowControl|Delay 0.2)
  (Utilities|FlowControl|DoOnce false) ; enters at Reset
)

(event EventBeginPlay
  ;[0.4766 0 1] PlayerRef kriegen
  (bind _asbp_player (Utilities|Casting|CastToBP_Player (Game|Player|GetPlayerPawn 0)))
  (Variables|Default|SetPlayer _asbp_player))

(event Collision|EventActorBeginOverlap
  (params (OtherActor :type Actor%20Object%20Reference)))

(event EventTick
  (params (DeltaSeconds :type Float%20%28single-precision%29))
  ;[1 0.2344 0] Erst wenn der Spieler in range
  (if (Variables|Default|GetisPlayerInRange)
    ;[1 0 0.9844] Trap-Loop
    (Utilities|FlowControl|DoOnce false :!label _label
      (:Completed
        (Utilities|FlowControl|Delay (* (Variables|Default|GetLooptime) 2.0))
        (Variables|Default|SetRelease true)
        (Utilities|FlowControl|Delay (Variables|Default|GetLooptime))
        (Variables|Default|SetRelease false)
        (goto _label Reset)))))

(fn ConstructionScript)