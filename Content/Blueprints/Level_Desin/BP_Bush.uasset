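; BP_Bush is a level bush with a flipbook sprite that reacts to being damaged.
; The first damage event sets an IsHit flag and plays a 2D foliage-hit sound, and further hits are ignored until Respawn clears the flag.
; The construction script swaps in the second bush's idle flipbook when IsBush02 is set.
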(event Game|Damage|EventAnyDamage
  (params (Damage :type Float%20%28single-precision%29) (DamageType :type Damage%20Type%20Object%20Reference) (InstigatedBy :type Controller%20Object%20Reference) (DamageCauser :type Actor%20Object%20Reference))
  (if (not (Variables|Default|GetisHit))
    (Variables|Default|SetisHit true)
    ;[1 0.9375 0] Sound
    (Class|FMODBlueprintStatics|PlayEvent2D "/Game/FMOD/Events/BushDestroy_Foliage__Hit__Small_Tree.BushDestroy_Foliage__Hit__Small_Tree")))

(event EventRespawn
  (Variables|Default|SetisHit false))

(event EventBeginPlay
  (Variables|Default|SetisHit false))

(fn ConstructionScript
  (if (Variables|Default|GetisBush02)
    (Sprite|SetFlipbook (Variables|Default|GetSprite) "/Game/Sprites/Assets/Busch2/FB_Busch02_Idle_Asset.FB_Busch02_Idle_Asset")))