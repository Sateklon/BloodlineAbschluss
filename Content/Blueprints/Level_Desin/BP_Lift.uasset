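; BP_Lift is a lift that BP_Player operates from an onboard lever or call levers at the top and bottom.
; Overlaps show a button prompt and register the lift for interaction; each call lever does so only with the lift at the other end.
; Interact, ignored while moving, animates the active lever's flipbook, waits, then flips a timeline lerping the platform's Z toward TargetZValue or back.
; TargetZValue's sign sets the starting up/down state.
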(event OnComponentBeginOverlap(InteractionBox)
  (params (OverlappedComponent :type Primitive%20Component%20Object%20Reference) (OtherActor :type Actor%20Object%20Reference) (OtherComp :type Primitive%20Component%20Object%20Reference) (OtherBodyIndex :type Integer) (bFromSweep :type Boolean) (SweepResult :type Hit%20Result%20Structure%20%28by%20ref%29))
  ;[1 0 0.5859] Interaction vom Lift Selbst
  (bind _asbp_player (Utilities|Casting|CastToBP_Player OtherActor))
  (Default|PlayerCanInteract _asbp_player self)
  (Rendering|SetVisibility (Variables|Default|GetInteractionButton) true false)
  (Variables|Default|SetCurrentHebel 0))

(event OnComponentEndOverlap(InteractionBox)
  (params (OverlappedComponent :type Primitive%20Component%20Object%20Reference) (OtherActor :type Actor%20Object%20Reference) (OtherComp :type Primitive%20Component%20Object%20Reference) (OtherBodyIndex :type Integer))
  ;[1 0 0.5859] Interaction vom Lift Selbst
  (bind _asbp_player (Utilities|Casting|CastToBP_Player OtherActor))
  (Default|PlayerCannotInteract _asbp_player)
  (Rendering|SetVisibility (Variables|Default|GetInteractionButton) false false))

(event OnComponentBeginOverlap(DownHEBEL)
  (params (OverlappedComponent :type Primitive%20Component%20Object%20Reference) (OtherActor :type Actor%20Object%20Reference) (OtherComp :type Primitive%20Component%20Object%20Reference) (OtherBodyIndex :type Integer) (bFromSweep :type Boolean) (SweepResult :type Hit%20Result%20Structure%20%28by%20ref%29))
  ;[0 1 0.2031] HebelDown
  (bind _asbp_player (Utilities|Casting|CastToBP_Player OtherActor))
  (if (Variables|Default|GetisLiftUp)
    (Default|PlayerCanInteract _asbp_player self)
    (Rendering|SetVisibility (Variables|Default|GetInteractionButtonDown) true false)
    (Variables|Default|SetCurrentHebel 1)))

(event OnComponentEndOverlap(DownHEBEL)
  (params (OverlappedComponent :type Primitive%20Component%20Object%20Reference) (OtherActor :type Actor%20Object%20Reference) (OtherComp :type Primitive%20Component%20Object%20Reference) (OtherBodyIndex :type Integer))
  ;[0 1 0.2031] HebelDown
  (bind _asbp_player (Utilities|Casting|CastToBP_Player OtherActor))
  (Default|PlayerCannotInteract _asbp_player)
  (Rendering|SetVisibility (Variables|Default|GetInteractionButtonDown) false false))

(event OnComponentBeginOverlap(UpHEBEL)
  (params (OverlappedComponent :type Primitive%20Component%20Object%20Reference) (OtherActor :type Actor%20Object%20Reference) (OtherComp :type Primitive%20Component%20Object%20Reference) (OtherBodyIndex :type Integer) (bFromSweep :type Boolean) (SweepResult :type Hit%20Result%20Structure%20%28by%20ref%29))
  ;[0.2656 0 1] HebelUp
  (bind _asbp_player (Utilities|Casting|CastToBP_Player OtherActor))
  (if (not (Variables|Default|GetisLiftUp))
    (Default|PlayerCanInteract _asbp_player self)
    (Rendering|SetVisibility (Variables|Default|GetInteractionButtonUP) true false)
    (Variables|Default|SetCurrentHebel 2)))

(event OnComponentEndOverlap(UpHEBEL)
  (params (OverlappedComponent :type Primitive%20Component%20Object%20Reference) (OtherActor :type Actor%20Object%20Reference) (OtherComp :type Primitive%20Component%20Object%20Reference) (OtherBodyIndex :type Integer))
  ;[0.2656 0 1] HebelUp
  (bind _asbp_player (Utilities|Casting|CastToBP_Player OtherActor))
  (Default|PlayerCannotInteract _asbp_player)
  (Rendering|SetVisibility (Variables|Default|GetInteractionButtonUP) false false))

(event Custom|HebelAnim
  (bind _hebel (Variables|Default|GetHebel))
  (bind _hebel1 (Variables|Default|GetHebel1))
  (bind _hebel2 (Variables|Default|GetHebel2))
  ;[1 0.3047 0] HebelAnim
  (switch int (Variables|Default|GetCurrentHebel)
    (:0
      (Utilities|FlowControl|FlipFlop
        (:A
          (Sprite|SetFlipbook _hebel "/Game/Sprites/Useables/FB_Hebel_ActivateLEFT.FB_Hebel_ActivateLEFT"))
        (:B
          (Sprite|SetFlipbook _hebel "/Game/Sprites/Useables/FB_Hebel_ActivateRIGHT.FB_Hebel_ActivateRIGHT")))
      (Components|Timeline|PlayfromStart (Variables|Default|GetHebel)))
    (:1
      (Utilities|FlowControl|FlipFlop
        (:A
          (Sprite|SetFlipbook _hebel1 "/Game/Sprites/Useables/FB_Hebel_ActivateLEFT.FB_Hebel_ActivateLEFT"))
        (:B
          (Sprite|SetFlipbook _hebel1 "/Game/Sprites/Useables/FB_Hebel_ActivateRIGHT.FB_Hebel_ActivateRIGHT")))
      (Components|Timeline|PlayfromStart (Variables|Default|GetHebel1)))
    (:2
      (Utilities|FlowControl|FlipFlop
        (:A
          (Sprite|SetFlipbook _hebel2 "/Game/Sprites/Useables/FB_Hebel_ActivateLEFT.FB_Hebel_ActivateLEFT"))
        (:B
          (Sprite|SetFlipbook _hebel2 "/Game/Sprites/Useables/FB_Hebel_ActivateRIGHT.FB_Hebel_ActivateRIGHT")))
      (Components|Timeline|PlayfromStart (Variables|Default|GetHebel2)))))

(event Custom|HebelFlipbookSetup
  ;[0.9453 1 0] SetupHebel
  (Components|Timeline|SetLooping (Variables|Default|GetHebel) false)
  (Components|Timeline|SetLooping (Variables|Default|GetHebel1) false)
  (Components|Timeline|SetLooping (Variables|Default|GetHebel2) false))

(event EventBeginPlay
  ;[0.5703 1 0] StartLogik, wo befindet sich der Lift
  (CallFunction|HebelFlipbookSetup)
  (if (< (Variables|Default|GetTargetZValue) 0.0)
    (Variables|Default|SetisLiftUp true)
    (else
      (Variables|Default|SetisLiftUp false))))

(event EventInteract
  ;[1 0.2578 0] Lift oder Hebel nur Interagierbar, solang der Lift in Ruhelage ist
  (if (not (Variables|Default|GetisMoving))
    (CallFunction|HebelAnim)
    (Utilities|FlowControl|Delay 1.0)
    ;[0 1 0.25] Ist der Lift Oben ? Nein, dann ist er es, wenn ja, dann nicht
    (if (Variables|Default|GetisLiftUp)
      (Variables|Default|SetisLiftUp false)
      (else
        (Variables|Default|SetisLiftUp true)))
    ;[0.1719 1 0] LiftMovement
    (Utilities|FlowControl|FlipFlop
      (:A
        (bind _alpha (Timeline|BesseresLiftMovement Play)
          (:Update
            (Variables|Default|SetisMoving true)
            (Transformation|SetRelativeLocation (Variables|Default|GetPlattform) (Math|Vector|MakeVector 0.0 0.0 (Math|Float|Lerp 0.0 (Variables|Default|GetTargetZValue) _alpha)) false false))
          (:Finished
            (Variables|Default|SetisMoving false))))
      (:B
        (Timeline|BesseresLiftMovement Reverse)))))

(fn ConstructionScript)