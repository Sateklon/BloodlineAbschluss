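; BP_HealthPotion is a pickup that adds one health potion to the game mode's count when the player touches it.
; It caches GM_Plattformer on BeginPlay and filters overlaps to BP_Player.
; An overlap calls Collect, which updates the potion count through the game mode and destroys the actor, then plays a 2D pickup sound.
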(event EventBeginPlay
  (bind _asgm_plattformer (Utilities|Casting|CastToGM_Plattformer (Game|GetGameMode)))
  (Variables|Default|SetGameMode _asgm_plattformer))

(event Collision|EventActorBeginOverlap
  (params (OtherActor :type Actor%20Object%20Reference))
  ;[0.4072 0 0.1812] Collected der Player ?
  (bind _asbp_player (Utilities|Casting|CastToBP_Player OtherActor))
  (if true
    (CallFunction|Collect _asbp_player)
    ;;[0.6875 1 0] Sound
    (Class|FMODBlueprintStatics|PlayEvent2D "/Game/FMOD/Events/Collect02_Cutlery__Hit_Dish.Collect02_Cutlery__Hit_Dish")))

(event EventCollect
  (params (Collector :type Pawn%20Object%20Reference))
  ;[0.4072 0 0.1812] Dann mach Dinge
  (Default|UpdateHealthpotions (Variables|Default|GetGameMode) 1)
  (Actor|DestroyActor))

(fn ConstructionScript)