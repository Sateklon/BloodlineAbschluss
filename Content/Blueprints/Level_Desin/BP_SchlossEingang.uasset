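; BP_SchlossEingang is a castle entrance door built from Paper2D flipbooks that opens when the player approaches.
; A back layer (RenderComponent) and a front layer (VorderesSprite) loop their initial flipbooks from BeginPlay.
; When player pawn 0 overlaps the Trigger, the door collision is disabled and both layers switch to their entrance flipbooks with looping off.
; Nothing in the graph closes the door again.
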(event OnComponentBeginOverlap(Trigger)
  (params (OverlappedComponent :type Primitive%20Component%20Object%20Reference) (OtherActor :type Actor%20Object%20Reference) (OtherComp :type Primitive%20Component%20Object%20Reference) (OtherBodyIndex :type Integer) (bFromSweep :type Boolean) (SweepResult :type Hit%20Result%20Structure%20%28by%20ref%29))
  (bind _vorderes_sprite (Variables|Default|GetVorderes%20Sprite))
  (bind _rendercomponent (Variables|Default|GetRenderComponent))
  (if (== OtherActor (Game|Player|GetPlayerPawn 0))
    (Collision|SetCollisionEnabled (Variables|Default|GetTürCollision) "NoCollision")
    (Utilities|FlowControl|Sequence
      (:then_0
        (Sprite|SetFlipbook _rendercomponent "/Game/Sprites/Useables/FB_SchlossEingang_Hinten.FB_SchlossEingang_Hinten")
        (Components|Timeline|SetLooping _rendercomponent false))
      (:then_1
        (Sprite|SetFlipbook _vorderes_sprite "/Game/Sprites/Useables/FB_SchlossEingangVorne.FB_SchlossEingangVorne")
        (Components|Timeline|SetLooping _vorderes_sprite false)))))

(event EventBeginPlay
  (Components|Timeline|SetLooping (Variables|Default|GetRenderComponent) true)
  (Components|Timeline|SetLooping (Variables|Default|GetVorderes%20Sprite) true))

(fn ConstructionScript)