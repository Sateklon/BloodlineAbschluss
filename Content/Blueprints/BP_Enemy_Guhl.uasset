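; Guhl enemy Blueprint that switches between walking and running based on aggro range and has a charge lunge.
; Tick checks IsInAggroRange and uses two cross-resetting DoOnce gates, so walk speed is doubled or restored to its base only once per state change.
; GuhlCharge launches the character horizontally along the world X axis, choosing the direction from the sign of its forward vector's X.
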(event Custom|GuhlCharge
  ;[0.6641 1 0] ChargeLaunch
  (Character|LaunchCharacter (Math|Vector|MakeVector (Math|Interpolation|Ease "Linear" 1.0 0.0 (Math|Float|SelectFloat 5e+02 -5e+02 (>= (.x (Transformation|GetActorForwardVector)) 0.0))) 0.0 0.0) false false))

(event EventBeginPlay
  (|CallParentFunction) ; This node is disabled and will not be called.\nDrag off pins to build functionality.
)

(event Collision|EventActorBeginOverlap
  (params (OtherActor :type Actor%20Object%20Reference)))

(event EventTick
  (params (DeltaSeconds :type Float%20%28single-precision%29))
  (bind _charactermovement (Variables|Character|GetCharacterMovement))
  ;[1 0 0.4687] RunCheck
  (|CallParentFunction DeltaSeconds)
  (if (Variables|Default|GetisInAggroRange)
    ;;[0.8281 1 0] Run
    (Utilities|FlowControl|Sequence
      (:then_0
        (goto _label_2 Reset))
      (:then_1
        (Utilities|FlowControl|DoOnce false :!label _label
          (:Completed
            (Variables|/Script/Engine.CharacterMovementComponent|SetMaxWalkSpeed _charactermovement (* (Variables|/Script/Engine.CharacterMovementComponent|GetMaxWalkSpeed _charactermovement) 2.0))))))
    (else
      ;;[1 0.09375 0] Walk
      (Utilities|FlowControl|Sequence
        (:then_0
          (goto _label Reset))
        (:then_1
          (Utilities|FlowControl|DoOnce false :!label _label_2
            (:Completed
              (Variables|/Script/Engine.CharacterMovementComponent|SetMaxWalkSpeed (Variables|Character|GetCharacterMovement) 2e+02))))))))

(fn ConstructionScript
  (|CallParentFunction))