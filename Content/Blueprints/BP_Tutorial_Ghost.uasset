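; Tutorial ghost actor that fades in with a whoosh and shows a text box while the player is inside its trigger area.
; BeginPlay hides the WBP_TutorialTextBox widget and sets its button icon.
; On overlap, a sprite-alpha timeline leads into looping delays that type two texts letter by letter, revealing the icon between them.
; Leaving interrupts typing, fades the ghost out and starts a brief cooldown against retriggering.
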(event OnComponentBeginOverlap(TutorialArea)
  (params (OverlappedComponent :type Primitive%20Component%20Object%20Reference) (OtherActor :type Actor%20Object%20Reference) (OtherComp :type Primitive%20Component%20Object%20Reference) (OtherBodyIndex :type Integer) (bFromSweep :type Boolean) (SweepResult :type Hit%20Result%20Structure%20%28by%20ref%29))
  (bind _sprite (Variables|Default|GetSprite))
  (bind _returnvalue (Class|PaperFlipbookComponent|GetSpriteColor _sprite))
  ;[0.3594 0 1] Player betritt die Tutorial Area
  (if (== OtherActor (Game|Player|GetPlayerPawn 0))
    ;[0.8047 1 0] CleanUP
    (Variables|Default|SetDisplayText1 "")
    (Variables|Default|SetDisplayText2 "")
    (if (not (Variables|Default|GetIsTutorialCooldown))
      (Variables|Default|SetIsInTutorialTrigger true)
      ;;[1 0 0.75] leere den text einmal
      (Rendering|Components|TextRender|SetText (Variables|Default|GetTutorial%20Text%201) "")
      (Utilities|FlowControl|Delay 0.2)
      ;[1 0.1406 0] Sound
      (Class|FMODBlueprintStatics|PlayEvent2D "/Game/FMOD/Events/TutorialGhost_ES_PREL_Whoosh_Flicker_-_SFX_Producer.TutorialGhost_ES_PREL_Whoosh_Flicker_-_SFX_Producer")
      ;[1 0.9844 0] Show Tutorial
      (bind _alpha (Timeline|FadeIN PlayFromStart)
        (:Update
          (Sprite|SetSpriteColor _sprite (Utilities|Struct|MakeLinearColor (.r _returnvalue) (.g _returnvalue) (.b _returnvalue) (Math|Float|Lerp 0.0 1.0 _alpha))))
        (:Finished
          (Rendering|SetVisibility (Variables|Default|GetTutorialBox) true false)
          ;[0.6406 1 0] Text 1 typing
          ;;[1 0.1406 0] Type, bis der Text da ist
          (Utilities|FlowControl|Delay 0.05 :!label _label)
          (Utilities|FlowControl|Sequence
            (:then_0
              ;;[0.8281 1 0] Typing Text
              (bind _output_get (Variables|Default|SetDisplayText1 (Utilities|String|GetSubstring (Utilities|String|ToString(Text) (Variables|Default|GetTutorialText1)) 0 (+ (Utilities|String|Len (Variables|Default|GetDisplayText1)) 1))))
              (Rendering|Components|TextRender|SetText (Variables|Default|GetTutorial%20Text%201) (Utilities|Text|ToText(String) _output_get)))
            (:then_1
              (if (Utilities|Enum|Equal(Enum) (Utilities|String|ToString(Text) (Variables|Default|GetTutorialText1)) (Variables|Default|GetDisplayText1))
                (Variables|/Script/UMG.Widget|SetVisibility (Variables|Default|GetUI_Button1) "Visible")
                ;[1 0.6328 0] Type Text 1 Over, Show Button
                (Variables|/Script/UMG.Widget|SetVisibility (Variables|Default|GetTutorial%20Text%202) "Visible")
                ;[0.6406 1 0] Text 2 typing
                ;;[1 0.1406 0] Type, bis der Text da ist
                (Utilities|FlowControl|Delay 0.05 :!label _label_2)
                (Utilities|FlowControl|Sequence
                  (:then_0
                    ;;[0.8281 1 0] Typing Text
                    (bind _output_get_2 (Variables|Default|SetDisplayText2 (Utilities|String|GetSubstring (Utilities|String|ToString(Text) (Variables|Default|GetTutorialText2)) 0 (+ (Utilities|String|Len (Variables|Default|GetDisplayText2)) 1))))
                    (Rendering|Components|TextRender|SetText (Variables|Default|GetTutorial%20Text%202) (Utilities|Text|ToText(String) _output_get_2)))
                  (:then_1
                    (if (not (Utilities|Enum|Equal(Enum) (Utilities|String|ToString(Text) (Variables|Default|GetTutorialText2)) (Variables|Default|GetDisplayText2)))
                      (if (Variables|Default|GetIsInTutorialTrigger)
                        (goto _label_2)
                        (else
                          ;;[0.9922 0 1] Interupded
                          (Rendering|Components|TextRender|SetText (Variables|Default|GetTutorial%20Text%201) "...")
                          (Rendering|Components|TextRender|SetText (Variables|Default|GetTutorial%20Text%202) "")
                          (Variables|/Script/UMG.Widget|SetVisibility (Variables|Default|GetUI_Button1) "Collapsed"))))))
                (elif (Variables|Default|GetIsInTutorialTrigger)
                  (goto _label)
                  (else
                    ;;[0.9922 0 1] Interupded
                    (Rendering|Components|TextRender|SetText (Variables|Default|GetTutorial%20Text%201) "...")
                    (Variables|/Script/UMG.Widget|SetVisibility (Variables|Default|GetUI_Button1) "Collapsed")))))))))))

(event OnComponentEndOverlap(TutorialArea)
  (params (OverlappedComponent :type Primitive%20Component%20Object%20Reference) (OtherActor :type Actor%20Object%20Reference) (OtherComp :type Primitive%20Component%20Object%20Reference) (OtherBodyIndex :type Integer))
  (bind _sprite (Variables|Default|GetSprite))
  (bind _tutorial_text_2 (Variables|Default|GetTutorial%20Text%202))
  (bind _returnvalue (Class|PaperFlipbookComponent|GetSpriteColor _sprite))
  ;[1 0 0.7266] Player verlässt die TutorialArea
  (if (== OtherActor (Game|Player|GetPlayerPawn 0))
    ;[0 0.7656 1] CleanUP
    (if (Variables|Default|GetIsInTutorialTrigger)
      (Variables|Default|SetIsInTutorialTrigger false)
      (Variables|Default|SetIsTutorialCooldown true)
      ;;[1 0 0.75] leere den text einmal
      (Rendering|Components|TextRender|SetText (Variables|Default|GetTutorial%20Text%201) "...")
      (Rendering|Components|TextRender|SetText _tutorial_text_2 "")
      (Variables|/Script/UMG.Widget|SetVisibility _tutorial_text_2 "Collapsed")
      (Variables|/Script/UMG.Widget|SetVisibility (Variables|Default|GetUI_Button1) "Collapsed")
      (Utilities|FlowControl|Delay 0.2)
      ;[0 0.3906 1] HideTutorial
      (bind _alpha (Timeline|FadeOut PlayFromStart)
        (:Update
          (Sprite|SetSpriteColor _sprite (Utilities|Struct|MakeLinearColor (.r _returnvalue) (.g _returnvalue) (.b _returnvalue) (Math|Float|Lerp 1.0 0.0 _alpha))))
        (:Finished
          (Rendering|SetVisibility (Variables|Default|GetTutorialBox) false false)
          (Variables|Default|SetDisplayText1 "")
          (Variables|Default|SetDisplayText2 "")
          (Utilities|FlowControl|Delay 1.0)
          (Variables|Default|SetIsTutorialCooldown false))))))

(event EventBeginPlay
  ;[0 0.03906 1] Setup
  (bind _aswbp_tutorial_text_box (Utilities|Casting|CastToWBP_TutorialTextBox (UserInterface|GetWidget (Variables|Default|GetTutorialBox))))
  (Variables|Default|SetWBP%20Tutorial%20Text%20Box _aswbp_tutorial_text_box)
  (Variables|Default|SetTutorial%20Text%201 (Variables|/Game/Blueprints/UI/WBP_TutorialTextBox.WBP_TutorialTextBox_C|GetTutorialText1 _aswbp_tutorial_text_box))
  (Variables|Default|SetTutorial%20Text%202 (Variables|/Game/Blueprints/UI/WBP_TutorialTextBox.WBP_TutorialTextBox_C|GetTutorialText2 _aswbp_tutorial_text_box))
  (Variables|Default|SetUI_Button1 (Variables|/Game/Blueprints/UI/WBP_TurorialButtonSprite.WBP_TurorialButtonSprite_C|GetSprite (Variables|/Game/Blueprints/UI/WBP_TutorialTextBox.WBP_TutorialTextBox_C|GetUI_Button1 _aswbp_tutorial_text_box)))
  ;[0 1 0.8828] Hide Tutorial
  (Rendering|SetVisibility (Variables|Default|GetTutorialBox) false false)
  (Class|CommonLazyImage|SetBrushfromLazyTexture (Variables|Default|GetUI_Button1) (Variables|Default|GetDesiredTutorialButton) false)
  ;[1 0 0.75] leere den text einmal
  (Rendering|Components|TextRender|SetText (Variables|Default|GetTutorial%20Text%201) "")
  (Variables|/Script/UMG.Widget|SetVisibility (Variables|Default|GetUI_Button1) "Collapsed"))

(fn ConstructionScript
  ;[0 0.03906 1] Construct
  (bind _aswbp_tutorial_text_box (Utilities|Casting|CastToWBP_TutorialTextBox (UserInterface|GetWidget (Variables|Default|GetTutorialBox))))
  (Rendering|Components|TextRender|SetText (Variables|/Game/Blueprints/UI/WBP_TutorialTextBox.WBP_TutorialTextBox_C|GetTutorialText1 _aswbp_tutorial_text_box) (Variables|Default|GetTutorialText1))
  (Rendering|Components|TextRender|SetText (Variables|/Game/Blueprints/UI/WBP_TutorialTextBox.WBP_TutorialTextBox_C|GetTutorialText2 _aswbp_tutorial_text_box) (Variables|Default|GetTutorialText2)))