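; BP_Interactable is an interactable actor that shows a sprite prompt when BP_Player is in range.
; Box overlaps register or clear it with the player and toggle the PaperSprite, skipping registration once it has been used.
; Interact hides the sprite and marks it used, then after a short delay re-arms it if repeat interaction is allowed.
; An unconnected save-system snippet for listing chests never runs.
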(event OnComponentBeginOverlap(Box)
  (params (OverlappedComponent :type Primitive%20Component%20Object%20Reference) (OtherActor :type Actor%20Object%20Reference) (OtherComp :type Primitive%20Component%20Object%20Reference) (OtherBodyIndex :type Integer) (bFromSweep :type Boolean) (SweepResult :type Hit%20Result%20Structure%20%28by%20ref%29))
  (if (not (Variables|Default|GetPlayerHasInteracted))
    (bind _asbp_player (Utilities|Casting|CastToBP_Player OtherActor))
    (Default|PlayerCanInteract _asbp_player self)
    (Rendering|SetVisibility (Variables|Default|GetPaperSprite) true false)))

(event OnComponentEndOverlap(Box)
  (params (OverlappedComponent :type Primitive%20Component%20Object%20Reference) (OtherActor :type Actor%20Object%20Reference) (OtherComp :type Primitive%20Component%20Object%20Reference) (OtherBodyIndex :type Integer))
  ;[0.1953 0 1] Player darf nicht mehr interagieren
  (bind _asbp_player (Utilities|Casting|CastToBP_Player OtherActor))
  (Default|PlayerCannotInteract _asbp_player)
  (Rendering|SetVisibility (Variables|Default|GetPaperSprite) false false))

(event EventBeginPlay)

(event Collision|EventActorBeginOverlap
  (params (OtherActor :type Actor%20Object%20Reference)))

(event EventTick
  (params (DeltaSeconds :type Float%20%28single-precision%29)))

(event EventInteract
  ;[0.6641 0 1] Interaction
  (Variables|Default|SetPlayerHasInteracted true)
  (Rendering|SetVisibility (Variables|Default|GetPaperSprite) false false)
  (Utilities|FlowControl|Delay 0.2)
  (Variables|Default|SetPlayerHasInteracted (not (Variables|Default|GetCanMoretimeInteract))))

(fn ConstructionScript)