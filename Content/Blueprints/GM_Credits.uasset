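; GM_Credits is the game mode for the credits screen, setting up its UI on BeginPlay.
; It creates the WBP_Main widget, adds it to the viewport and puts WBP_Credits on its menu stack.
; It switches input to UI only with the mouse cursor hidden.
; After a short delay it also sends the credits widget to the HUD through PushToMenuStackMessage.
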(event EventBeginPlay
  (bind _returnvalue (Game|GetPlayerController 0))
  ;[0 0.25 1] UI erzeugen
  (bind _returnvalue_2 (UserInterface|CreateWidget "/Game/Blueprints/UI/WBP_Main.WBP_Main_C"))
  (UserInterface|Viewport|AddtoViewport _returnvalue_2 0)
  (bind _output_get (Variables|Default|SetWBP_Main _returnvalue_2))
  (Class|CommonActivatableWidgetContainerBase|AddWidget (Variables|/Game/Blueprints/UI/WBP_Main.WBP_Main_C|GetMenuStack _output_get) "/Game/Blueprints/UI/WBP_Credits.WBP_Credits_C")
  (Input|SetInputModeUIOnly _returnvalue 0 "DoNotLock" false)
  (Variables|/Script/Engine.PlayerController|SetbShowMouseCursor _returnvalue false)
  (Utilities|FlowControl|Delay 0.2)
  (Class|BPIHUD|PushtoMenuStack(Message) (HUD|GetHUD _returnvalue) "/Game/Blueprints/UI/WBP_Credits.WBP_Credits_C"))

(event EventTick
  (params (DeltaSeconds :type Float%20%28single-precision%29)))

(fn ConstructionScript)