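; Paper2D lever for a lift floor that requests the lift to its Level when the player enters its Box.
; The overlap passes Level and itself to the parent BP_Lift_2 actor and shows a Button sprite, which hides again when the player leaves.
; HebelAnim alternates left and right activation flipbooks via FlipFlop, playing each once without looping; it is not called here, and LiftFailRequest is an empty stub.
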(event OnComponentBeginOverlap(Box)
  (params (OverlappedComponent :type Primitive%20Component%20Object%20Reference) (OtherActor :type Actor%20Object%20Reference) (OtherComp :type Primitive%20Component%20Object%20Reference) (OtherBodyIndex :type Integer) (bFromSweep :type Boolean) (SweepResult :type Hit%20Result%20Structure%20%28by%20ref%29))
  (bind _returnvalue (Actor|GetParentActor))
  ;[1 0 0.8672] Etagenknopf wird erreicht
  (if (== OtherActor (Game|Player|GetPlayerPawn 0))
    (Utilities|IsValid _returnvalue
      (:Is%20Valid
        (bind _asbp_lift_2 (Utilities|Casting|CastToBP_Lift_2 _returnvalue))
        (Default|LevelRequest _asbp_lift_2 (Variables|Default|GetLevel) self)
        (CallFunction|ShowButton)))))

(event OnComponentEndOverlap(Box)
  (params (OverlappedComponent :type Primitive%20Component%20Object%20Reference) (OtherActor :type Actor%20Object%20Reference) (OtherComp :type Primitive%20Component%20Object%20Reference) (OtherBodyIndex :type Integer))
  (if (== OtherActor (Game|Player|GetPlayerPawn 0))
    (CallFunction|HideButton)))

(event Custom|LiftFailRequest
  ;[0 0.7891 1] Lift ist schon da
)

(event Custom|Show%20Button
  ;[1 0.8203 0] ButtonVisibility
  (Rendering|SetVisibility (Variables|Default|GetButton) true false))

(event Custom|Hide%20Button
  ;[1 0.8203 0] ButtonVisibility
  (Rendering|SetVisibility (Variables|Default|GetButton) false false))

(event Custom|HebelAnim
  (bind _rendercomponent (Variables|Default|GetRenderComponent))
  ;[0.1953 0 1] HebelAnim
  (Utilities|FlowControl|FlipFlop
    (:A
      (Sprite|SetFlipbook _rendercomponent "/Game/Sprites/Useables/Flipbooks/FB_Hebel_ActivateLEFT.FB_Hebel_ActivateLEFT"))
    (:B
      (Sprite|SetFlipbook _rendercomponent "/Game/Sprites/Useables/Flipbooks/FB_Hebel_ActivateRIGHT.FB_Hebel_ActivateRIGHT")))
  (Components|Timeline|PlayfromStart _rendercomponent))

(event EventBeginPlay
  (Components|Timeline|SetLooping (Variables|Default|GetRenderComponent) false))

(fn ConstructionScript)