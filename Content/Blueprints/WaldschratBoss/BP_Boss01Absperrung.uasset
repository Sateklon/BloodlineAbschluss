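; A boss-room barrier for the Waldschrat boss, built from a flipbook sprite and a collision box that blocks passage during the fight.
; The construction script picks the gate or boss-room flipbook based on IsBoss2.
; The box starts without collision; PlayAnim enables it after a short delay and sets ON, while Reset disables it and clears ON.
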(event Custom|PlayAnim
  ;[1 0.7969 0] Sperr ab
  (Utilities|FlowControl|Delay 0.5)
  (Variables|Default|SetON true)
  (Collision|SetCollisionEnabled (Variables|Default|GetBox) "QueryAndPhysics"))

(event Custom|Reset
  (Variables|Default|SetON false)
  (Collision|SetCollisionEnabled (Variables|Default|GetBox) "NoCollision"))

(event EventBeginPlay
  ;[0 0.5312 1] Start "Idle"
  (Collision|SetCollisionEnabled (Variables|Default|GetBox) "NoCollision")
  (if (Variables|Default|GetIsBoss2)
    _))

(event Collision|EventActorBeginOverlap
  (params (OtherActor :type Actor%20Object%20Reference)))

(event EventTick
  (params (DeltaSeconds :type Float%20%28single-precision%29)))

(fn ConstructionScript
  (if (Variables|Default|GetIsBoss2)
    (Sprite|SetFlipbook (Variables|Default|GetRenderComponent) "/Game/Sprites/Useables/FB_GateAbsperrung.FB_GateAbsperrung")
    (else
      (Sprite|SetFlipbook (Variables|Default|GetRenderComponent) "/Game/Sprites/Enemys/Flipbooks/FB_BossRaum.FB_BossRaum"))))