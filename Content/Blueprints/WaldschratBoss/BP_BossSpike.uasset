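; BP_BossSpike is a spike hazard for the Waldschrat boss that damages the player when it strikes.
; On Strike it checks actors overlapping its Damagebox and applies SpikeDamage to player 0 through a DoOnce, reset after a one-second delay to limit repeat hits.
; A debris and dirt sound event node exists in the graph but never runs.
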(event Custom|Strike
  (for _array_element (Collision|GetOverlappingActors (Variables|Default|GetDamagebox) "/Script/Engine.Actor" :!class /Script/Engine.PrimitiveComponent)
    (if (== _array_element (Game|Player|GetPlayerPawn 0))
      (Utilities|FlowControl|DoOnce false
        (:Completed
          (Game|Damage|ApplyDamage _array_element (Variables|Default|GetSpikeDamage) 0 self)))))
  (Utilities|FlowControl|Delay 1.0)
  (Utilities|FlowControl|DoOnce false) ; enters at Reset
)

(event EventBeginPlay)

(fn ConstructionScript)