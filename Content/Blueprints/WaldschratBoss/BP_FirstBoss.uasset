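; First boss of the 2D platformer (Waldschrat): walks, turns toward the player and resets when they die.
; Tick drives movement, charge damage and a random attack roll; externally triggered events perform melee hits, tendril and spike spawns, and charges.
; Damage feeds a delayed-drain health bar and stacking bleed.
; Activation and death switch music and UI; victory awards souls, unlocks the achievement and destroys the arena barriers.
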(event OnComponentBeginOverlap(BossIdleArea)
  (params (OverlappedComponent :type Primitive%20Component%20Object%20Reference) (OtherActor :type Actor%20Object%20Reference) (OtherComp :type Primitive%20Component%20Object%20Reference) (OtherBodyIndex :type Integer) (bFromSweep :type Boolean) (SweepResult :type Hit%20Result%20Structure%20%28by%20ref%29))
  ;[0 0.3203 1] BossidleTrigger
  (bind _player (Variables|Default|GetPlayer)
    (:then
      (if (== _player OtherActor)
        (if (not (Variables|AttackVariables|GetCharging))
          (Variables|Default|SetBossCanIdle true))))
    (:else)))

(event OnComponentBeginOverlap(TopDamageBox)
  (params (OverlappedComponent :type Primitive%20Component%20Object%20Reference) (OtherActor :type Actor%20Object%20Reference) (OtherComp :type Primitive%20Component%20Object%20Reference) (OtherBodyIndex :type Integer) (bFromSweep :type Boolean) (SweepResult :type Hit%20Result%20Structure%20%28by%20ref%29))
  ;[0 0.9531 1] Geweih
  (if (== OtherActor (Variables|Default|GetPlayer))
    (Game|Damage|ApplyDamage OtherActor 2e+01 0 self "/Game/Blueprints/Data/BP_DamageNormal.BP_DamageNormal_C")))

(event OnComponentEndOverlap(BossIdleArea)
  (params (OverlappedComponent :type Primitive%20Component%20Object%20Reference) (OtherActor :type Actor%20Object%20Reference) (OtherComp :type Primitive%20Component%20Object%20Reference) (OtherBodyIndex :type Integer))
  ;[0 0.3203 1] BossidleTrigger
  (bind _player (Variables|Default|GetPlayer)
    (:then
      (if (== _player OtherActor)
        (if (not (Variables|AttackVariables|GetCharging))
          (Variables|Default|SetBossCanIdle false))))
    (:else)))

(event OnComponentEndOverlap(GroundCheck)
  (params (OverlappedComponent :type Primitive%20Component%20Object%20Reference) (OtherActor :type Actor%20Object%20Reference) (OtherComp :type Primitive%20Component%20Object%20Reference) (OtherBodyIndex :type Integer))
  ;[0 1 0.7422] GroundCheck
  (if (Variables|AttackVariables|GetCharging)
    ;;[1 0.3984 0] Charge to End
    (Utilities|FlowControl|DoOnce false :!label _label
      (:Completed
        (Variables|AttackVariables|SetisChargeOutOfArea true)
        (Pawn|Input|AddMovementInput "0, 0, 0" 0.0 false)
        (Utilities|FlowControl|Delay 2.0)
        (Variables|AttackVariables|SetCharging false)
        (Variables|AttackVariables|SetisChargeOutOfArea false)
        (CallFunction|AttackOver)
        (goto _label Reset)))
    (else
      ;;[0.7109 0 1] Turn Arround
      (CallFunction|Turnaround))))

(event OnComponentBeginOverlap(WalCheck)
  (params (OverlappedComponent :type Primitive%20Component%20Object%20Reference) (OtherActor :type Actor%20Object%20Reference) (OtherComp :type Primitive%20Component%20Object%20Reference) (OtherBodyIndex :type Integer) (bFromSweep :type Boolean) (SweepResult :type Hit%20Result%20Structure%20%28by%20ref%29))
  ;[1 0.09375 0] TileChecking
  (if (Variables|AttackVariables|GetCharging)
    ;;[1 0.6984 0] Charge to End
    (Utilities|FlowControl|DoOnce false :!label _label
      (:Completed
        (Variables|AttackVariables|SetisChargeOutOfArea true)
        (Pawn|Input|AddMovementInput "0, 0, 0" 0.0 false)
        (Utilities|FlowControl|Delay 2.0)
        (Variables|AttackVariables|SetCharging false)
        (Variables|AttackVariables|SetisChargeOutOfArea false)
        (CallFunction|AttackOver)
        (goto _label Reset)))
    (else
      ;;[0 0.2969 1] Turn Arround
      (CallFunction|Turnaround))))

(event Custom|Movement
  ;[0.6406 1 0] Movement
  (if (Variables|Default|GetisBossActivated)
    (if (and (not (Variables|Default|GetisDamageing)) (not (Variables|Default|GetisDead)))
      (if (not (Variables|AttackVariables|GetisAttacking))
        (if (not (Variables|Default|GetBossCanIdle))
          (if (not (Variables|AttackVariables|GetisChargeOutOfArea))
            (Pawn|Input|AddMovementInput (Transformation|GetActorForwardVector) 1.0 false)
            ;[0.6406 0 1] Rotate to Player
            (bind _player (Variables|Default|GetPlayer)
              (:then
                (if (not (Variables|AttackVariables|GetCharging))
                  (if (<= (.x (Transformation|GetActorLocation)) (.x (Transformation|GetActorLocation _player)))
                    (if (< (.x (Transformation|GetActorForwardVector)) 0.0)
                      (CallFunction|Turnaround))
                    (elif (not (< (.x (Transformation|GetActorForwardVector)) 0.0))
                      (CallFunction|Turnaround)))))
              (:else))))))))

(event Custom|BloodDamage
  ;[1 0 0.04741] BloodDamage System
  ;;[1 0 0.8203] Wird schon Blutschaden gemacht ?
  (if (and (not (Variables|BloodDamageSystem|GetisBloodmakingDamage)) (not (Variables|AttackVariables|GetBossIsSlayed)))
    ;;[0 0.6016 1] Blood an machen
    (Rendering|SetVisibility (Variables|Default|GetBloodDamageSprite) true false)
    (Utilities|FlowControl|Sequence
      (:then_0
        ;;[0.5234 1 0] Zähl die Stacks hoch
        (bind _output_get (Variables|BloodDamageSystem|SetBlood%20Stacks (+ (Variables|BloodDamageSystem|GetBlood%20Stacks) 1)))
        (if (>= _output_get 2)
          (Variables|BloodDamageSystem|SetisBloodmakingDamage true)))
      (:then_1
        ;;[0.6875 0 1] Stack anzeigen
        (Rendering|Components|Sprite|SetSprite (Variables|Default|GetBloodDamageSprite) (Utilities|Array|Get(acopy) (Variables|BloodDamageSystem|GetBlood%20Stack%20Sprites) (Variables|BloodDamageSystem|GetBlood%20Stacks))))
      (:then_2
        ;;[0.2422 0 1] nocjhmal checken ob alle stacks da sind
        (if (Variables|BloodDamageSystem|GetisBloodmakingDamage)
          ;;[0 0.3672 1] Der eigentliche Blutschaden
          (Utilities|FlowControl|Delay 2.0)
          (Game|Damage|ApplyDamage self (Variables|/Game/Blueprints/GM_Plattformer.GM_Plattformer_C|GetCurrentBloodDamage (Variables|Default|GetGameManager)) 0 0 "/Game/Blueprints/Data/BP_DamageBlood.BP_DamageBlood_C")
          (Class|FMODBlueprintStatics|PlayEvent2D "/Game/FMOD/Events/BloodDamage_ES_Intestines_Remove_2_-_SFX_Producer.BloodDamage_ES_Intestines_Remove_2_-_SFX_Producer")
          (Utilities|FlowControl|Delay 1.0)
          (Variables|BloodDamageSystem|SetBlood%20Stacks -1)
          (Variables|BloodDamageSystem|SetisBloodmakingDamage false)
          (Rendering|SetVisibility (Variables|Default|GetBloodDamageSprite) false false))))))

(event Custom|Attack01Over
  ;[0 1 0.6953] AttackOver
  (Variables|AttackVariables|SetBossAttack false)
  (if (<= (Variables|AttackVariables|GetAttackNumber) 1)
    (Utilities|FlowControl|Delay 1.5)
    (else
      (Utilities|FlowControl|Delay 0.5)))
  (CallFunction|AttackOver)
  (Utilities|FlowControl|Sequence
    (:then_0
      ;[0.5938 0 1] Attack01
      ;;[0.8516 1 0] Attack01
      (Utilities|FlowControl|DoOnce false) ; enters at Reset
    )
    (:then_1
      ;[0 0.9531 1] Attack02
      ;;[0 1 0.3672] Attack02
      (Utilities|FlowControl|DoOnce false) ; enters at Reset
    )))

(event Custom|SetupBossStartValues
  ;[0 0.6719 1] StartTarnsform
  (Variables|Default|SetBossTransform (Transformation|GetActorTransform)))

(event Custom|SingleSpike
  ;[0 1 0.4609] SpAttack01
  ;;[0.5 0 1] Single
  (bind _returnvalue (Game|SpawnActorfromClass "/Game/Blueprints/WaldschratBoss/BP_SingleTendril.BP_SingleTendril_C" (Math|Transform|MakeTransform (Transformation|GetWorldLocation (Variables|Default|GetSingleTedrilAttackSpawnpoint)) (Transformation|GetActorRotation) "1.000000,1.000000,1.000000") "AlwaysSpawn" "MultiplyWithRoot" 0 0))
  (Utilities|Array|Add (Variables|Default|GetAllTendrils) _returnvalue))

(event Custom|ResetBoss
  ;[0.9688 0 1] ResetBoss
  (Utilities|FlowControl|Delay 0.5)
  (Variables|Default|SetHealth (Variables|Default|GetMaxHealth))
  (Transformation|SetActorTransform (Variables|Default|GetBossTransform))
  (Variables|Default|SetisBossActivated false)
  (Variables|Default|SetisDamageing false)
  (Variables|Default|SetisDead false)
  (Variables|AttackVariables|SetisAttacking false)
  (Variables|AttackVariables|SetBossAttack false)
  (Variables|AttackVariables|SetCharging false)
  (Variables|AttackVariables|SetisChargeOutOfArea false)
  (Widget|SetVisibility (Variables|/Game/Blueprints/UI/WBP_Gameplay.WBP_Gameplay_C|GetWBP_WaldSchratBär_Healthbar (Variables|Default|GetWBP%20Gameplay)) "Collapsed")
  (Variables|BloodDamageSystem|SetBlood%20Stacks -1)
  (Rendering|SetVisibility (Variables|Default|GetBloodDamageSprite) false false)
  (CallFunction|AttackOver)
  (for _array_element (Variables|Default|GetAbsperrungen)
    (Utilities|IsValid _array_element
      (:Is%20Valid
        (bind _asbp_boss_01absperrung (Utilities|Casting|CastToBP_Boss01Absperrung _array_element))
        (Default|Reset _asbp_boss_01absperrung))))
  (if (not (Variables|AttackVariables|GetBossIsSlayed))
    (Class|FMODAudioComponent|SetEvent (Variables|/Script/FMODStudio.FMODAmbientSound|GetAudioComponent (Variables|Default|GetLevel%20Music)) "/Game/FMOD/Events/FirstLevel_ES_The_Last_Disaster_-_Howard_Harper-Barnes.FirstLevel_ES_The_Last_Disaster_-_Howard_Harper-Barnes")))

(event Custom|Attack02
  ;[0 0.9531 1] Attack02
  ;;[0 1 0.3672] Attack02
  (for _array_element (Collision|GetOverlappingActors (Variables|Default|GetAttack02Check) "/Script/Engine.Actor" :!class /Script/Engine.PrimitiveComponent)
    (if (== _array_element (Game|Player|GetPlayerPawn 0))
      (Utilities|FlowControl|DoOnce false
        (:Completed
          (Game|Damage|ApplyDamage _array_element (* (Variables|AttackVariables|GetAttackBaseDamage) 2.0) 0 self "/Game/Blueprints/Data/BP_DamageNormal.BP_DamageNormal_C"))))))

(event Custom|ParalaxDisable
  ;[0 0.625 1] ParalaxManager
  (bind _player (Variables|Default|GetPlayer)
    (:then
      (Rendering|SetVisibility (Variables|/Game/Blueprints/BP_Player.BP_Player_C|GetParalax%20Layer%208_BG _player) false false)
      (for _array_element (Components|GetChildrenComponents (Variables|/Game/Blueprints/BP_Player.BP_Player_C|GetParalax%20Layer%208_BG _player) false)
        (Rendering|SetVisibility _array_element false false)))
    (:else)))

(event Custom|ChargeDamageCheck
  ;[0.4062 0 1] ChargeAttack
  ;;[0.3125 1 0] Charge
  ;;;[1 0.8203 0] ChargeDamage
  (if (Variables|AttackVariables|GetCharging)
    (Utilities|FlowControl|Sequence
      (:then_0
        (for _array_element (Collision|GetOverlappingActors (Variables|Default|GetChargeDamageArea) "/Script/Engine.Actor" :!class /Script/Engine.PrimitiveComponent)
          (if (!= _array_element self)
            (Utilities|FlowControl|DoOnce false :!label _label
              (:Completed
                (Game|Damage|ApplyDamage _array_element 4e+01 0 self)
                (Utilities|FlowControl|Delay 0.5)
                (goto _label Reset))))))
      (:then_1
        ;;;;[0 1 0.6953] ChargeSpeed
        (if (Variables|AttackVariables|GetisChargeOutOfArea)
          (Variables|/Script/Engine.CharacterMovementComponent|SetMaxWalkSpeed (Variables|Character|GetCharacterMovement) 3e+02)
          (Utilities|FlowControl|DoOnce false :!label _label_2
            (:Completed
              (CallFunction|AttackOver)
              (Utilities|FlowControl|Delay 1.0)
              (goto _label_2 Reset)))
          (else
            (Variables|/Script/Engine.CharacterMovementComponent|SetMaxWalkSpeed (Variables|Character|GetCharacterMovement) 4.5e+02)))))))

(event Custom|2Spikes
  ;[1 0.3516 0] SpAttack01
  (if true
    ;;[0 0.8828 1] 2 Tendrils
    (bind _returnvalue (Game|SpawnActorfromClass "/Game/Blueprints/WaldschratBoss/BP_SingleTendril.BP_SingleTendril_C" (Math|Transform|MakeTransform (Transformation|GetWorldLocation (Variables|Default|GetSecondTendrilSpawn)) (Transformation|GetActorRotation) "1.000000,1.000000,1.000000") "AlwaysSpawn" "MultiplyWithRoot" 0 0))
    (Utilities|Array|Add (Variables|Default|GetAllTendrils) _returnvalue)
    (bind _returnvalue_2 (Game|SpawnActorfromClass "/Game/Blueprints/WaldschratBoss/BP_SingleTendril.BP_SingleTendril_C" (Transformation|GetWorldTransform (Variables|Default|GetSingleTedrilAttackSpawnpoint)) "Undefined" "MultiplyWithRoot" 0 0))
    (Utilities|Array|Add (Variables|Default|GetAllTendrils) _returnvalue_2)
    (else
      ;;[0.1953 1 0] Trigger  AOE Atack
      (if (== (Variables|AttackVariables|GetAttackNumber) 4)
        (CallFunction|AOEAttack)))))

(event Custom|SlayedBoss
  (bind _level_music (Variables|Default|GetLevel%20Music))
  (bind _wbp_gameplay (Variables|Default|GetWBP%20Gameplay))
  (bind _wbp_gameplay_2 (Variables|Default|GetWBP%20Gameplay))
  (bind _youwintext (Variables|/Game/Blueprints/UI/WBP_Gameplay.WBP_Gameplay_C|GetYouWinText _wbp_gameplay))
  (bind _youwintext_2 (Variables|/Game/Blueprints/UI/WBP_Gameplay.WBP_Gameplay_C|GetYouWinText _wbp_gameplay_2))
  (bind _colorandopacity (Variables|/Script/UMG.TextBlock|GetColorAndOpacity _youwintext_2))
  (bind _colorandopacity_2 (Variables|/Script/UMG.TextBlock|GetColorAndOpacity _youwintext))
  ;[0 1 1] Slayed the Boss
  (Variables|AttackVariables|SetBossIsSlayed true)
  (Rendering|SetVisibility (Variables|Default|GetBloodDamageSprite) false false)
  (bind _alpha (Timeline|You%20Win Play)
    (:Update
      (Appearance|SetColorandOpacity _youwintext_2 (Utilities|Struct|MakeSlateColor (Utilities|Struct|MakeLinearColor (.r (.specifiedcolor _colorandopacity)) (.g (.specifiedcolor _colorandopacity)) (.b (.specifiedcolor _colorandopacity)) (Math|Float|Lerp 0.0 1.0 _alpha)) (.coloruserule _colorandopacity)) :!class /Script/UMG.TextBlock))
    (:Finished
      (Variables|/Script/UMG.Widget|SetVisibility (Variables|/Game/Blueprints/UI/WBP_Gameplay.WBP_Gameplay_C|GetWBP_WaldSchratBär_Healthbar (Variables|Default|GetWBP%20Gameplay)) "Collapsed")
      (Utilities|FlowControl|Delay 2.0)
      (bind _alpha_2 (Timeline|YouWinOut Play)
        (:Update
          (Appearance|SetColorandOpacity _youwintext (Utilities|Struct|MakeSlateColor (Utilities|Struct|MakeLinearColor (.r (.specifiedcolor _colorandopacity_2)) (.g (.specifiedcolor _colorandopacity_2)) (.b (.specifiedcolor _colorandopacity_2)) (Math|Float|Lerp 1.0 0.0 _alpha_2)) (.coloruserule _colorandopacity_2)) :!class /Script/UMG.TextBlock))
        (:Finished
          (Default|UpdateSouls (Variables|Default|GetGameManager) (Variables|Default|GetSeelenwert))
          ;;[1 0 0.2578] SteamAchievment
          (Default|SlayBoss01 (Variables|Default|GetGameManager))
          (CallFunction|DeactivateBoss)
          (Utilities|IsValid _level_music
            (:Is%20Valid
              (Class|FMODAudioComponent|SetEvent (Variables|/Script/FMODStudio.FMODAmbientSound|GetAudioComponent _level_music) "/Game/FMOD/Events/FirstLevel_ES_The_Last_Disaster_-_Howard_Harper-Barnes.FirstLevel_ES_The_Last_Disaster_-_Howard_Harper-Barnes")
              (Utilities|FlowControl|Sequence
                (:then_0
                  (for _array_element (Variables|Default|GetAbsperrungen)
                    (Actor|DestroyActor _array_element))
                  (Collision|SetCollisionEnabled (Variables|Collision|GetCapsuleComponent) "NoCollision")
                  (Utilities|FlowControl|Delay 0.2)
                  (Actor|DestroyActor))))))))))

(event Custom|AOEAttack
  ;[0.2188 0 1] SPAttack03
  ;;[0 1 0.25] AOE Attack
  (for _array_element (Variables|AttackVariables|GetGeAllSpikeSpawns)
    (Game|SpawnActorfromClass "/Game/Blueprints/WaldschratBoss/BP_BossSpike.BP_BossSpike_C" (Transformation|GetActorTransform _array_element) "Undefined" "MultiplyWithRoot" 0 0)))

(event Custom|DeactivateBoss
  ;[1 0 0.4922] Deactivate Boss
  ;;[1 0 0.2812] mach die healthbar aus
  (Default|DeactivateBosshealthbar (Variables|Default|GetWBP%20Gameplay))
  (if (not (Variables|AttackVariables|GetBossIsSlayed))
    (Variables|Default|SetisBossActivated false)
    (CallFunction|ResetBoss)))

(event Custom|Channeling
  ;[1 0 0.4453] Channeling
  (Utilities|FlowControl|Delay 2.0)
  (Variables|AttackVariables|SetisChanneling false))

(event Custom|ActivateBoss
  ;[1 0 0.4453] Activate Boss
  (if (not (Variables|Default|GetisBossActivated))
    (if (not (Variables|AttackVariables|GetBossIsSlayed))
      ;;[1 0 0.6797] Player trigger Boss
      (Variables|Default|SetisBossActivated true)
      (Default|ActivateBossHealthBar (Variables|Default|GetWBP%20Gameplay) (Variables|Default|GetBossName))
      ;;[0.8047 0 1] Setup BossHealthbar
      (Progress|SetPercent (Variables|/Game/Blueprints/UI/WBP_WaldSchratBär_Healthbar.WBP_WaldSchratBär_Healthbar_C|GetCurrentHealthbar (Variables|/Game/Blueprints/UI/WBP_Gameplay.WBP_Gameplay_C|GetWBP_WaldSchratBär_Healthbar (Variables|Default|GetWBP%20Gameplay))) (/ (Variables|Default|GetHealth) (Variables|Default|GetMaxHealth)))
      (CallFunction|ParalaxDisable)
      (bind _asbp_player (Utilities|Casting|CastToBP_Player (Game|Player|GetPlayerPawn 0)))
      (Variables|Default|SetPlayer _asbp_player)
      (if (not (Variables|AttackVariables|GetBossIsSlayed))
        (Class|FMODAudioComponent|SetEvent (Variables|/Script/FMODStudio.FMODAmbientSound|GetAudioComponent (Variables|Default|GetLevel%20Music)) "/Game/FMOD/Events/FisrtBoss_ES_Halls_of_Titans_-_Hampus_Naeselius.FisrtBoss_ES_Halls_of_Titans_-_Hampus_Naeselius")))))

(event Custom|Attack01
  ;[0.5938 0 1] Attack01
  ;;[0.8516 1 0] Attack01
  (for _array_element (Collision|GetOverlappingActors (Variables|Default|GetAttack01Check) "/Script/Engine.Actor" :!class /Script/Engine.PrimitiveComponent)
    (if (== _array_element (Game|Player|GetPlayerPawn 0))
      (Utilities|FlowControl|DoOnce false
        (:Completed
          (Game|Damage|ApplyDamage _array_element (Variables|AttackVariables|GetAttackBaseDamage) 0 self "/Game/Blueprints/Data/BP_DamageNormal.BP_DamageNormal_C"))))))

(event Custom|UpdatePrevHB
  (bind _wbp_gameplay (Variables|Default|GetWBP%20Gameplay))
  (bind _maxhealth (Variables|Default|GetMaxHealth))
  (bind _wbp_waldschratbär_healthbar (Variables|/Game/Blueprints/UI/WBP_Gameplay.WBP_Gameplay_C|GetWBP_WaldSchratBär_Healthbar _wbp_gameplay))
  ;[0 1 0.3672] DamageingBoss
  (Variables|Default|SetTakenDamage 0.0)
  ;;[0.8281 1 0] HelthbarUpdate
  (Widget|SetVisibility (Variables|/Game/Blueprints/UI/WBP_WaldSchratBär_Healthbar.WBP_WaldSchratBär_Healthbar_C|GetDamagetake _wbp_waldschratbär_healthbar) "Collapsed")
  ;;;[1 0 0.09375] MatheSören
  (bind _alpha (Timeline|Drop%20Health PlayFromStart)
    (:Update
      (Progress|SetPercent (Variables|/Game/Blueprints/UI/WBP_WaldSchratBär_Healthbar.WBP_WaldSchratBär_Healthbar_C|GetPrevHealthbar _wbp_waldschratbär_healthbar) (Math|Float|Lerp (/ (Variables|Default|GetHealthBeforeDamage) _maxhealth) (/ (Variables|Default|GetHealth) _maxhealth) _alpha)))
    (:Finished
      (CallFunction|SetupNextHB))))

(event Custom|ParalaxEnable
  ;[0 0.625 1] ParalaxManager
  (bind _player (Variables|Default|GetPlayer)
    (:then
      (Rendering|SetVisibility (Variables|/Game/Blueprints/BP_Player.BP_Player_C|GetParalax%20Layer%208_BG _player) true false)
      (for _array_element (Components|GetChildrenComponents (Variables|/Game/Blueprints/BP_Player.BP_Player_C|GetParalax%20Layer%208_BG _player) false)
        (Rendering|SetVisibility _array_element true false)))
    (:else)))

(event Custom|SetupNextHB
  ;[0 1 0.3672] DamageingBoss
  (Utilities|FlowControl|DoOnce false) ; enters at Reset
)

(event Custom|AttackRotation
  ;[0.1484 1 0] AttackSetup
  (if (Variables|Default|GetisBossActivated)
    (if (and (not (Variables|Default|GetisDamageing)) (not (Variables|Default|GetisDead)))
      (if (not (Variables|AttackVariables|GetisAttacking))
        (Utilities|FlowControl|DoOnce false
          (:Completed
            (Utilities|FlowControl|Delay (Math|Random|RandomFloatinRange 1.0 3.0))
            (bind _output_get (Variables|AttackVariables|SetAttackNumber (Math|Random|RandomInteger 12)))
            (Variables|AttackVariables|SetisAttacking true)
            (if (>= _output_get 10)
              (Variables|AttackVariables|SetisChanneling true))
            (Variables|AttackVariables|SetBossAttack true)))))))

(event Custom|Turnaround
  ;[1 0.8438 0] Turn arround
  (Transformation|SetActorRotation (Math|Rotator|CombineRotators (Transformation|GetActorRotation) "0.000000,180.000000,0.000000")))

(event Custom|AttackOver
  ;[0.1484 1 0] AttackSetup
  (Variables|AttackVariables|SetisAttacking false)
  (Variables|AttackVariables|SetBossAttack false)
  (Utilities|FlowControl|DoOnce false) ; enters at Reset
)

(event Custom|ChargeAttack
  ;[0.4062 0 1] ChargeAttack
  ;;[0.3125 1 0] Charge
  ;;;[0.875 1 0] Setup before Charge // Channel before Charge
  (Variables|AttackVariables|SetisAttacking false)
  (Variables|AttackVariables|SetCharging true))

(event Custom|Attack02Over
  ;[0 1 0.6953] AttackOver
  (Variables|AttackVariables|SetBossAttack false)
  (if (<= (Variables|AttackVariables|GetAttackNumber) 1)
    (Utilities|FlowControl|Delay 1.5)
    (else
      (Utilities|FlowControl|Delay 0.5)))
  (CallFunction|AttackOver)
  (Utilities|FlowControl|Sequence
    (:then_0
      ;[0.5938 0 1] Attack01
      ;;[0.8516 1 0] Attack01
      (Utilities|FlowControl|DoOnce false) ; enters at Reset
    )
    (:then_1
      ;[0 0.9531 1] Attack02
      ;;[0 1 0.3672] Attack02
      (Utilities|FlowControl|DoOnce false) ; enters at Reset
    )))

(event EventBeginPlay
  ;[1 0.5156 0] Setup
  (CallFunction|SetupBossStartValues)
  (bind _asgm_plattformer (Utilities|Casting|CastToGM_Plattformer (Game|GetGameMode)))
  (bind _output_get (Variables|Default|SetGameManager _asgm_plattformer))
  (bind _aswbp_gameplay (Utilities|Casting|CastToWBP_Gameplay (Class|CommonActivatableWidgetContainerBase|GetActiveWidget (Variables|/Game/Blueprints/UI/WBP_Main.WBP_Main_C|GetGameplayStack (Variables|/Game/Blueprints/GM_Plattformer.GM_Plattformer_C|GetWBP_Main _output_get)))))
  (Variables|Default|SetWBP%20Gameplay _aswbp_gameplay)
  (Variables|Default|SetHealth (Variables|Default|GetMaxHealth))
  (bind _asbp_player (Utilities|Casting|CastToBP_Player (Game|Player|GetPlayerPawn 0)))
  (Variables|Default|SetPlayer _asbp_player))

(event EventTick
  (params (DeltaSeconds :type Float%20%28single-precision%29))
  ;[0.2422 0 1] Tick
  (if (Variables|Default|GetisBossActivated)
    (if (not (Variables|AttackVariables|GetBossIsSlayed))
      (CallFunction|Movement)
      (CallFunction|AttackRotation)
      (CallFunction|ChargeDamageCheck)
      ;;[0 0.4141 1] IsPlayerDead ?
      (bind _player (Variables|Default|GetPlayer)
        (:then
          (if (Variables|/Game/Blueprints/BP_Player.BP_Player_C|GetisDead _player)
            _
            (else
              (goto _label Reset))))
        (:else
          _))
      (Utilities|FlowControl|DoOnce false :!label _label
        (:Completed
          (Utilities|FlowControl|Delay 1.5)
          (CallFunction|ResetBoss))))))

(event Game|Damage|EventAnyDamage
  (params (Damage :type Float%20%28single-precision%29) (DamageType :type Damage%20Type%20Object%20Reference) (InstigatedBy :type Controller%20Object%20Reference) (DamageCauser :type Actor%20Object%20Reference))
  (bind _wbp_gameplay (Variables|Default|GetWBP%20Gameplay))
  (bind _wbp_waldschratbär_healthbar (Variables|/Game/Blueprints/UI/WBP_Gameplay.WBP_Gameplay_C|GetWBP_WaldSchratBär_Healthbar _wbp_gameplay))
  ;[0 1 0.3672] DamageingBoss
  (if (not (Variables|AttackVariables|GetBossIsSlayed))
    (if (== (Utilities|GetClass DamageType) "/Game/Blueprints/Data/BP_DamageBlood.BP_DamageBlood_C")
      (CallFunction|BloodDamage))
    (Variables|Default|SetTakenDamage (+ Damage (Variables|Default|GetTakenDamage)))
    (Utilities|FlowControl|Sequence
      (:then_0
        (Utilities|FlowControl|DoOnce false
          (:Completed
            (Variables|Default|SetHealthBeforeDamage (Variables|Default|GetHealth)))))
      (:then_1
        (bind _output_get (Variables|Default|SetHealth (- (Variables|Default|GetHealth) Damage)))
        (if (<= _output_get 0.0)
          (Variables|Default|SetisDead true)
          (CallFunction|SlayedBoss)
          (else
            (Variables|Default|SetisDamageing true)))
        (Progress|SetPercent (Variables|/Game/Blueprints/UI/WBP_WaldSchratBär_Healthbar.WBP_WaldSchratBär_Healthbar_C|GetCurrentHealthbar _wbp_waldschratbär_healthbar) (/ (Variables|Default|GetHealth) (Variables|Default|GetMaxHealth)))
        (Progress|SetPercent (Variables|/Game/Blueprints/UI/WBP_WaldSchratBär_Healthbar.WBP_WaldSchratBär_Healthbar_C|GetPrevHealthbar _wbp_waldschratbär_healthbar) (/ (Variables|Default|GetHealthBeforeDamage) (Variables|Default|GetMaxHealth)))
        (Widget|SetVisibility (Variables|/Game/Blueprints/UI/WBP_WaldSchratBär_Healthbar.WBP_WaldSchratBär_Healthbar_C|GetDamagetake _wbp_waldschratbär_healthbar) "Visible")
        (Rendering|Components|TextRender|SetText (Variables|/Game/Blueprints/UI/WBP_WaldSchratBär_Healthbar.WBP_WaldSchratBär_Healthbar_C|GetDamageNumber _wbp_waldschratbär_healthbar) (Utilities|Text|ToText(Float) (Variables|Default|GetTakenDamage) "HalfToEven"))
        ;;[0 0.6719 1] Stoppe den gegner
        (Pawn|Input|AddMovementInput "1.000000,0.000000,0.000000" 0.0 false)
        (Utilities|FlowControl|Delay 0.2)
        (Camera|PlayWorldCameraShake "/Game/Blueprints/BP_CameraShake_Damage.BP_CameraShake_Damage_C" (Transformation|GetActorLocation (Pawn|GetViewTarget (Game|GetPlayerController 0))) 0.0 2e+02)
        (Game|Feedback|ClientPlayForceFeedback (Game|GetPlayerController 0) "/Game/Blueprints/ControllerVibration/PlayerAttackHitVoibration.PlayerAttackHitVoibration" "None" false false false)
        (Class|FMODBlueprintStatics|PlayEvent2D "/Game/FMOD/Events/HitEnemy_Swipe__Hit_Body__Impact__Hard__Squelch.HitEnemy_Swipe__Hit_Body__Impact__Hard__Squelch")
        ;;[0 0.9297 1] Play Damage(or DeathAnim)
        (Class|PaperZDAnimInstance|JumptoNode (Variables|/Script/PaperZD.PaperZDAnimationComponent|GetAnimInstance (Variables|Default|GetAnimationComponent)) "Damageing" "None")
        (Utilities|Time|SetTimerbyEvent (delegate Custom|UpdatePrevHB) 1.5)))))

(fn ConstructionScript)