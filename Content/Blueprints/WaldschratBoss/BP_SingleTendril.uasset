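; BP_SingleTendril is a Waldschrat boss attack: a self-propelled tendril character that creeps straight along its forward vector and hurts the player.
; It spawns its own controller and plays a wood-creak sound, then adds movement input every tick.
; Each tick also checks the Thornes overlaps, damaging the player with a short DoOnce cooldown.
; It destroys itself on lifetime expiry, TileCheck overlap or NotGrounded; the tick ground check does nothing.
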(event OnComponentBeginOverlap(TileCheck)
  (params (OverlappedComponent :type Primitive%20Component%20Object%20Reference) (OtherActor :type Actor%20Object%20Reference) (OtherComp :type Primitive%20Component%20Object%20Reference) (OtherBodyIndex :type Integer) (bFromSweep :type Boolean) (SweepResult :type Hit%20Result%20Structure%20%28by%20ref%29))
  (Actor|DestroyActor))

(event Custom|SetupLifetime
  ;[1 0 0.2812] Lifetime
  (Utilities|FlowControl|Delay (Variables|Default|GetLifetime))
  (Actor|DestroyActor))

(event Custom|NotGrounded
  ;[1 0 0.2812] Lifetime
  (Actor|DestroyActor))

(event Custom|DamageCheck
  ;[0.3359 1 0] DamageRotation
  (for _array_element (Collision|GetOverlappingActors (Variables|Default|GetThornes) "/Script/Engine.Actor" :!class /Script/Engine.PrimitiveComponent)
    (if (== _array_element (Game|Player|GetPlayerPawn 0))
      (Utilities|FlowControl|DoOnce false :!label _label
        (:Completed
          (Game|Damage|ApplyDamage _array_element 2e+01 0 self)
          (Utilities|FlowControl|Delay 0.5)
          (goto _label Reset))))))

(event EventBeginPlay
  ;[1 0 0.4922] Setup
  (Pawn|SpawnDefaultController)
  (CallFunction|SetupLifetime)
  (Class|FMODBlueprintStatics|PlayEvent2D "/Game/FMOD/Events/Tendril_debris-wood-wood-creak-01.Tendril_debris-wood-wood-creak-01"))

(event EventTick
  (params (DeltaSeconds :type Float%20%28single-precision%29))
  ;[0.03125 1 0] Movement
  (Pawn|Input|AddMovementInput (Transformation|GetActorForwardVector) 1.0 false)
  (CallFunction|DamageCheck)
  ;[1 0 0.6797] Groundcheck
  (if (AI|Components|NavMovement|IsMovingonGround (Variables|Character|GetCharacterMovement))
    _))

(fn ConstructionScript)