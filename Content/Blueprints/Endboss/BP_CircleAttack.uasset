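; BP_CircleAttack is an endboss attack that plays a non-looping animation and creates an expanding circle that damages the player.
; Two timelines grow the DamageZone and slightly smaller SafeZone spheres, forming a ring.
; DamageZone overlap applies the externally set damage through a DoOnce unless SafeZone overlap has already flagged the player safe, a flag never cleared.
; With a valid BP_Endboss, the actor destroys itself after a short delay or when the boss dies.
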(event OnComponentBeginOverlap(DamageZone)
  (params (OverlappedComponent :type Primitive%20Component%20Object%20Reference) (OtherActor :type Actor%20Object%20Reference) (OtherComp :type Primitive%20Component%20Object%20Reference) (OtherBodyIndex :type Integer) (bFromSweep :type Boolean) (SweepResult :type Hit%20Result%20Structure%20%28by%20ref%29))
  ;[0.5469 1 0] DamageZone
  (if (== OtherActor (Game|Player|GetPlayerPawn 0))
    (if (not (Variables|Default|GetisPlayerSafe))
      (Utilities|FlowControl|DoOnce false
        (:Completed
          (Game|Damage|ApplyDamage OtherActor (Variables|Default|GetDamage) 0 0)))
      (else
        (Utilities|FlowControl|DoOnce false)))))

(event OnComponentBeginOverlap(SafeZone)
  (params (OverlappedComponent :type Primitive%20Component%20Object%20Reference) (OtherActor :type Actor%20Object%20Reference) (OtherComp :type Primitive%20Component%20Object%20Reference) (OtherBodyIndex :type Integer) (bFromSweep :type Boolean) (SweepResult :type Hit%20Result%20Structure%20%28by%20ref%29))
  ;[0 1 0.03906] PlayerSafeZone
  (if (== OtherActor (Game|Player|GetPlayerPawn 0))
    (Variables|Default|SetisPlayerSafe true)))

(event Custom|CircleCollision
  ;[0 0.1797 1] Vergrößerungslogik
  (bind _alpha (Timeline|CicleColision PlayFromStart)
    (:Update
      (Components|Sphere|SetSphereRadius (Variables|Default|GetDamageZone) (Math|Float|Lerp 32.0 9e+02 _alpha) true))))

(event Custom|SafeSpace
  ;[0 0.1797 1] Vergrößerungslogik
  (bind _alpha (Timeline|Safe%20Col PlayFromStart)
    (:Update
      (Components|Sphere|SetSphereRadius (Variables|Default|GetSafeZone) (Math|Float|Lerp 0.0 8.5e+02 _alpha) true))))

(event Custom|SetCircleDamage
  (params (CircleDamage :type Float%20%28double-precision%29))
  ;[0.4062 0 1] SetupDamage
  (Variables|Default|SetDamage CircleDamage))

(event EventBeginPlay
  (Components|Timeline|SetLooping (Variables|Default|GetRenderComponent) false)
  (CallFunction|CircleCollision)
  (CallFunction|SafeSpace)
  (bind _returnvalue (Actor|GetActorOfClass "/Game/Blueprints/Endboss/BP_Endboss.BP_Endboss_C"))
  (bind _output_get (Variables|Default|SetEndboss _returnvalue))
  (Utilities|IsValid _output_get
    (:Is%20Valid
      (Utilities|FlowControl|Delay 4.0)
      (Actor|DestroyActor))))

(event EventTick
  (params (DeltaSeconds :type Float%20%28single-precision%29))
  (Utilities|IsValid (Variables|Default|GetEndboss)
    (:Is%20Valid
      (if (Variables|/Game/Blueprints/Endboss/BP_Endboss.BP_Endboss_C|GetisDead (Variables|Default|GetEndboss))
        (Utilities|FlowControl|DoOnce false
          (:Completed
            (Actor|DestroyActor)))))))

(fn ConstructionScript)