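; Projectile for the endboss that turns to face the player once at spawn and deals damage on overlap.
; Damage is passed in through SetupDamage and applied when the Trigger component overlaps the player.
; It destroys itself after a fixed delay, if no valid player exists at rotation setup, or when Tick sees that the endboss is dead.
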(event OnComponentBeginOverlap(Trigger)
  (params (OverlappedComponent :type Primitive%20Component%20Object%20Reference) (OtherActor :type Actor%20Object%20Reference) (OtherComp :type Primitive%20Component%20Object%20Reference) (OtherBodyIndex :type Integer) (bFromSweep :type Boolean) (SweepResult :type Hit%20Result%20Structure%20%28by%20ref%29))
  ;[1 0.1641 0] TriggerDamage
  (if (== OtherActor (Variables|Default|GetPlayer))
    (Game|Damage|ApplyDamage (Variables|Default|GetPlayer) (Variables|Default|GetDamage) 0 self)))

(event Custom|SetupDamage
  (params (ProjectileDamage :type Float%20%28double-precision%29))
  ;[0.6641 0 1] SetupDamage
  (Variables|Default|SetDamage ProjectileDamage))

(event Custom|SetupRotation
  (bind _player (Variables|Default|GetPlayer)
    (:then
      (Variables|Default|SetLookAtRotation (Math|Rotator|FindLookatRotation (Transformation|GetActorLocation) (Transformation|GetActorLocation _player)))
      (Transformation|SetActorRotation (Math|Rotator|FindLookatRotation (Transformation|GetActorLocation) (Transformation|GetActorLocation _player))))
    (:else
      (Actor|DestroyActor))))

(event EventBeginPlay
  (bind _asbp_player (Utilities|Casting|CastToBP_Player (Game|Player|GetPlayerPawn 0)))
  (Variables|Default|SetPlayer _asbp_player)
  (CallFunction|SetupRotation)
  (bind _returnvalue (Actor|GetActorOfClass "/Game/Blueprints/Endboss/BP_Endboss.BP_Endboss_C"))
  (bind _output_get (Variables|Default|SetEndboss _returnvalue))
  (Utilities|IsValid _output_get
    (:Is%20Valid
      _)
    (:Is%20Not%20Valid
      _))
  (Utilities|FlowControl|Delay 8.0)
  (Actor|DestroyActor))

(event EventTick
  (params (DeltaSeconds :type Float%20%28single-precision%29))
  (Utilities|IsValid (Variables|Default|GetEndboss)
    (:Is%20Valid
      (if (Variables|/Game/Blueprints/Endboss/BP_Endboss.BP_Endboss_C|GetisDead (Variables|Default|GetEndboss))
        (Utilities|FlowControl|DoOnce false
          (:Completed
            (Actor|DestroyActor)))))))

(fn ConstructionScript)