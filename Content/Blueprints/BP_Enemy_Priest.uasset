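; Priest enemy for a side-view platformer: patrols, faces the player within aggro range, attacks with aimed missiles or melee, and awards souls in its kill event.
; Overlap volumes and a timer drive turning and range flags; Tick handles movement, aim and a cooldown-gated attack flag, while shot, melee, kill and respawn events have no callers here.
; Damage updates the health bar and feedback; stacking dark damage triggers stunning burn ticks, while blood damage is an empty stub.
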(event OnComponentEndOverlap(GroundCheck)
  (params (OverlappedComponent :type Primitive%20Component%20Object%20Reference) (OtherActor :type Actor%20Object%20Reference) (OtherComp :type Primitive%20Component%20Object%20Reference) (OtherBodyIndex :type Integer))
  ;[0.05469 1 0] Groundcheck
  (CallFunction|Turnaround))

(event OnComponentBeginOverlap(WallCheck)
  (params (OverlappedComponent :type Primitive%20Component%20Object%20Reference) (OtherActor :type Actor%20Object%20Reference) (OtherComp :type Primitive%20Component%20Object%20Reference) (OtherBodyIndex :type Integer) (bFromSweep :type Boolean) (SweepResult :type Hit%20Result%20Structure%20%28by%20ref%29))
  ;[0 1 0.9766] Walcheck
  (CallFunction|Turnaround))

(event OnComponentBeginOverlap(Aggrorange)
  (params (OverlappedComponent :type Primitive%20Component%20Object%20Reference) (OtherActor :type Actor%20Object%20Reference) (OtherComp :type Primitive%20Component%20Object%20Reference) (OtherBodyIndex :type Integer) (bFromSweep :type Boolean) (SweepResult :type Hit%20Result%20Structure%20%28by%20ref%29))
  ;[0 1 0.1328] Aggrorange
  (if (== OtherActor (Game|Player|GetPlayerPawn 0))
    (Variables|Default|SetisInAggroRange true)))

(event OnComponentEndOverlap(Aggrorange)
  (params (OverlappedComponent :type Primitive%20Component%20Object%20Reference) (OtherActor :type Actor%20Object%20Reference) (OtherComp :type Primitive%20Component%20Object%20Reference) (OtherBodyIndex :type Integer))
  ;[0 1 0.1328] Aggrorange
  (if (== OtherActor (Game|Player|GetPlayerPawn 0))
    (Variables|Default|SetisInAggroRange false)))

(event OnComponentBeginOverlap(MeeleRange)
  (params (OverlappedComponent :type Primitive%20Component%20Object%20Reference) (OtherActor :type Actor%20Object%20Reference) (OtherComp :type Primitive%20Component%20Object%20Reference) (OtherBodyIndex :type Integer) (bFromSweep :type Boolean) (SweepResult :type Hit%20Result%20Structure%20%28by%20ref%29))
  ;[0.3828 0 1] Melerange
  (if (== OtherActor (Game|Player|GetPlayerPawn 0))
    (Variables|Default|SetisInMeleRange true)))

(event OnComponentEndOverlap(MeeleRange)
  (params (OverlappedComponent :type Primitive%20Component%20Object%20Reference) (OtherActor :type Actor%20Object%20Reference) (OtherComp :type Primitive%20Component%20Object%20Reference) (OtherBodyIndex :type Integer))
  ;[0.3828 0 1] Melerange
  (if (== OtherActor (Game|Player|GetPlayerPawn 0))
    (Variables|Default|SetisInMeleRange false)))

(event Custom|Movement
  ;[0 0.5312 1] KIMovement
  (if (and (and (not (Variables|Default|GetisInAggroRange)) (not (Variables|Default|GetisDead))) (not (Variables|Default|GetisStunned)))
    (if (not (Variables|Default|GetisAttacking))
      (Pawn|Input|AddMovementInput (Transformation|GetActorForwardVector) 1.0 false))))

(event Custom|Tracking%20Player
  ;[0 0.5547 1] Schussrichtung
  (bind _player (Variables|Default|GetPlayer)
    (:then
      (Transformation|SetRelativeRotation (Variables|Default|GetSpawnMissilePoint) (Math|Rotator|MakeRotator 0.0 (.pitch (Math|Rotator|FindLookatRotation (Transformation|GetWorldLocation (Variables|Default|GetSpawnMissilePoint)) (Transformation|GetActorLocation _player))) 0.0) false false))
    (:else
      (Transformation|SetRelativeRotation (Variables|Default|GetSpawnMissilePoint) "0, 0, 0" false false))))

(event Custom|BloodDamage)

(event Custom|DarkDamage
  ;[0 0.7422 1] Dark Damage
  (if (== (not (Variables|Default|GetIsDarkDamageMaking)) (not (Variables|Default|GetisDead)))
    (Rendering|SetVisibility (Variables|Default|GetDarkDamageSprite) true false)
    (Utilities|Time|SetTimerbyEvent (delegate Custom|DarkInpurCooldown) 3.0)
    (Utilities|FlowControl|Sequence
      (:then_0
        (bind _output_get (Variables|Default|SetDarkStacks (+ (Variables|Default|GetDarkStacks) 1)))
        (if (>= _output_get 2)
          (Variables|Default|SetIsDarkDamageMaking true)))
      (:then_1
        (Sprite|SetFlipbook (Variables|Default|GetDarkDamageSprite) (Utilities|Array|Get(acopy) (Variables|Default|GetDarkDamageSprites) (Variables|Default|GetDarkStacks))))
      (:then_2
        (if (Variables|Default|GetIsDarkDamageMaking)
          (Utilities|FlowControl|Delay 1.0)
          (if (> (Variables|Stats|GetCurrent%20Health) 0.0)
            (if (not (Variables|Default|GetIsDarkDamageCooldown))
              (Variables|Default|SetDarkStacks -1)
              (if (< (Variables|Default|GetDarkBurnStacks) (Variables|/Game/Blueprints/GM_Plattformer.GM_Plattformer_C|GetDarkDamageBaseStacks (Variables|Default|GetGameManager))) :!label _label
                (Game|Damage|ApplyDamage self (Variables|/Game/Blueprints/GM_Plattformer.GM_Plattformer_C|GetCurrentDarkDamage (Variables|Default|GetGameManager)) 0 0 "/Game/Blueprints/Data/BP_DamageDark.BP_DamageDark_C")
                (CallFunction|EnemyStuning)
                (Variables|Default|SetDarkBurnStacks (+ (Variables|Default|GetDarkBurnStacks) 1))
                (Utilities|FlowControl|Delay 0.2)
                (goto _label)
                (else
                  (Variables|Default|SetDarkBurnStacks 0)
                  (Utilities|FlowControl|Delay 0.2)
                  (Variables|Default|SetDarkStacks -1)
                  (Variables|Default|SetIsDarkDamageMaking false)
                  (Rendering|SetVisibility (Variables|Default|GetDarkDamageSprite) false false))))))))))

(event Custom|EnemyStuning
  ;[0 1 0.9766] Stun
  ;[1 0.3516 0] Enemy Stunning
  (if (Variables|Default|GetcanBeStunned)
    (Variables|Default|SetisStunned true)))

(event Custom|DarkInpurCooldown
  ;[0 0.7422 1] Dark Damage
  (Rendering|SetVisibility (Variables|Default|GetDarkDamageSprite) false false)
  (Variables|Default|SetDarkStacks -1))

(event Custom|TurnCheck
  (bind _returnvalue (Game|Player|GetPlayerPawn 0))
  ;[0 1 0.1328] Aggrorange
  (Utilities|IsValid _returnvalue
    (:Is%20Valid
      (if (Variables|Default|GetisInAggroRange)
        (if (> (.x (Transformation|GetActorLocation _returnvalue)) (.x (Transformation|GetActorLocation)))
          ;;[1 0.375 0] Turn
          (if (not (> (.x (Transformation|GetActorForwardVector)) 0.0))
            (CallFunction|Turnaround))
          (elif (< (.x (Transformation|GetActorLocation _returnvalue)) (.x (Transformation|GetActorLocation)))
            (if (not (< (.x (Transformation|GetActorForwardVector)) 0.0))
              (CallFunction|Turnaround))))))))

(event Custom|KillEnemy
  ;[0.6875 1 0] Priest Die
  (if (Variables|Default|GetisDead)
    (Variables|Default|SetIsDarkDamageMaking false)
    (bind _aswbp_enemy_health_bar (Utilities|Casting|CastToWBP_EnemyHealthBar (UserInterface|GetWidget (Variables|Default|GetHealtbar))))
    (Widget|SetVisibility _aswbp_enemy_health_bar "Collapsed")
    (Rendering|SetVisibility (Variables|Default|GetHealtbar) false false)
    (bind _asgm_plattformer (Utilities|Casting|CastToGM_Plattformer (Game|GetGameMode)))
    (Default|UpdateSouls _asgm_plattformer (Variables|Stats|GetSoulvalue))
    ;;[0.9688 1 0] für Achievment
    (Default|FirstEnemyKilled _asgm_plattformer)
    (Collision|SetCollisionEnabled (Variables|Default|GetCapsuleComponent) "NoCollision")
    ;;[0.5234 0 1] Absicherung
    (Variables|Default|SetisDead true)))

(event Custom|MeeleAttack
  ;[0 1 0.8125] MeeleAttack
  (if (not (Variables|Default|GetisDead))
    (for _array_element (Collision|GetOverlappingActors (Variables|Default|GetHitBox) "/Script/Engine.Actor" :!class /Script/Engine.PrimitiveComponent)
      (if (== _array_element (Game|Player|GetPlayerPawn 0))
        (Game|Damage|ApplyDamage _array_element (Variables|Stats|GetMeleDamage) 0 self "/Game/Blueprints/Data/BP_DamageNormal.BP_DamageNormal_C")))))

(event Custom|PriestSetup
  ;[1 0.6797 0] Setup
  (Variables|Default|SetStartposition (Transformation|GetActorLocation)))

(event Custom|Turnaround
  ;[1 0 0.6797] Turnarround
  (Transformation|SetActorRotation (Math|Rotator|CombineRotators (Transformation|GetActorRotation) "0.000000,180.000000,0.000000")))

(event Custom|EnemyTimer
  ;[1 0 0.3047] Enemy Timer für Patrulie
  (if (not (Variables|Default|GetisInAggroRange))
    (Utilities|FlowControl|Delay (Variables|Stats|GetPatroulieZeit))
    (if (and (AI|Components|NavMovement|IsMovingonGround (Variables|Character|GetCharacterMovement)) (not (Math|Float|NearlyEqual(Float) (.x (Transformation|GetVelocity)) 0.0 0.001)))
      (Utilities|FlowControl|DoOnce false :!label _label
        (:Completed
          (CallFunction|Turnaround)
          (Utilities|FlowControl|Delay 1.0)
          (Utilities|FlowControl|Sequence
            (:then_0
              (goto _label Reset))
            (:then_1
              (CallFunction|EnemyTimer)))))
      (else
        (CallFunction|EnemyTimer)))))

(event Custom|Shooting
  (bind _spawnmissilepoint (Variables|Default|GetSpawnMissilePoint))
  ;[0.1719 0 1] Shooting
  (if (not (Variables|Default|GetisDead))
    (bind _returnvalue (Game|SpawnActorfromClass "/Game/Blueprints/BP_PriestMissile.BP_PriestMissile_C" (Math|Transform|MakeTransform (Transformation|GetWorldLocation _spawnmissilepoint) (Transformation|GetWorldRotation _spawnmissilepoint) "1.000000,1.000000,1.000000") "Undefined" "MultiplyWithRoot" 0 0))
    (Utilities|IsValid _returnvalue
      (:Is%20Valid
        (Default|SetArrowDamage _returnvalue (Variables|Stats|GetRangeDamage))))))

(event Custom|Attack
  ;[0.6172 1 0] Attacking
  (if (Variables|Default|GetisInAggroRange)
    (if (not (Variables|Default|GetisAttacking))
      (Utilities|FlowControl|DoOnce false :!label _label
        (:Completed
          (Utilities|FlowControl|Delay 0.5)
          (Variables|Default|SetisAttacking true)
          (Utilities|FlowControl|Delay (Variables|Stats|GetAttackspeed))
          (goto _label Reset))))))

(event EventRespawn
  ;[0.9453 1 0] Respawn
  (Variables|Stats|SetCurrent%20Health (Variables|Stats|GetMaxHealth))
  (Variables|Default|SetisDead false)
  (bind _aswbp_enemy_health_bar (Utilities|Casting|CastToWBP_EnemyHealthBar (UserInterface|GetWidget (Variables|Default|GetHealtbar))))
  (Widget|SetVisibility _aswbp_enemy_health_bar "Collapsed")
  (Rendering|SetVisibility (Variables|Default|GetHealtbar) true false)
  (Transformation|SetActorLocation (Variables|Default|GetStartposition) false false)
  (Collision|SetCollisionEnabled (Variables|Default|GetCapsuleComponent) "QueryOnly")
  (Variables|Default|SetisDamaged false)
  (Variables|Default|SetisDead false)
  (bind _asbp_player (Utilities|Casting|CastToBP_Player (Game|Player|GetPlayerPawn 0)))
  (Variables|Default|SetPlayer _asbp_player))

(event EventTick
  (params (DeltaSeconds :type Float%20%28single-precision%29))
  (CallFunction|Movement)
  (CallFunction|Attack)
  (CallFunction|TrackingPlayer)
  (CallFunction|TurnCheck))

(event EventBeginPlay
  ;[1 0 0.1172] BeginnPlay
  (bind _asbp_player (Utilities|Casting|CastToBP_Player (Game|Player|GetPlayerPawn 0)))
  (Variables|Default|SetPlayer _asbp_player)
  (Variables|Stats|SetCurrent%20Health (Variables|Stats|GetMaxHealth))
  (CallFunction|EnemyTimer)
  (CallFunction|PriestSetup)
  (bind _asgm_plattformer (Utilities|Casting|CastToGM_Plattformer (Game|GetGameMode)))
  (Variables|Default|SetGameManager _asgm_plattformer)
  ;[0 0.6016 1] Blood aus machen
  (Rendering|SetVisibility (Variables|Default|GetBloodDamageSprite) false false))

(event Game|Damage|EventAnyDamage
  (params (Damage :type Float%20%28single-precision%29) (DamageType :type Damage%20Type%20Object%20Reference) (InstigatedBy :type Controller%20Object%20Reference) (DamageCauser :type Actor%20Object%20Reference))
  ;[0 1 0.2266] Take Damage
  ;;[1 0.9375 0] Player finden
  (bind _asbp_player (Utilities|Casting|CastToBP_Player (Game|Player|GetPlayerPawn 0)))
  (Variables|Default|SetPlayer _asbp_player)
  (if (and (not (== DamageCauser self)) (== (Utilities|GetClass DamageType) (Variables|Default|GetWoundableDamagetype)))
    (if (== (Variables|Default|GetWoundableDamagetype) (Variables|Default|GetBloodDamageClass))
      (CallFunction|BloodDamage)
      (elif (== (Variables|Default|GetWoundableDamagetype) (Variables|Default|GetDarkDamageClass))
        (CallFunction|DarkDamage))))
  ;;[1 0.2109 0] DamageMathe
  (if (not (Variables|Default|GetisDead))
    (Variables|Default|SetisAttacked true)
    (Variables|Default|SetHealthBeforeDamage (Variables|Stats|GetCurrent%20Health))
    (Variables|Default|SetTakenDamage (+ (Variables|Default|GetTakenDamage) Damage))
    (bind _output_get (Variables|Stats|SetCurrent%20Health (- (Variables|Stats|GetCurrent%20Health) Damage)))
    ;;[0.9688 0 1] Absicherung
    (if (<= _output_get 0.0)
      (Variables|Default|SetisDead true)
      (else
        ;;[0 1 0.625] Fancy Stuff
        (Variables|Default|SetisDamaged true)))
    (Camera|PlayWorldCameraShake "/Game/Blueprints/BP_CameraShake_Damage.BP_CameraShake_Damage_C" (Transformation|GetWorldLocation (Variables|/Game/Blueprints/BP_Player.BP_Player_C|GetCamera (Variables|Default|GetPlayer))) 0.0 2e+02)
    (Game|Feedback|ClientPlayForceFeedback (Game|GetPlayerController 0) "/Game/Blueprints/ControllerVibration/PlayerAttackHitVoibration.PlayerAttackHitVoibration" "None" false false false)
    (Class|FMODBlueprintStatics|PlayEvent2D "/Game/FMOD/Events/HitEnemy_Swipe__Hit_Body__Impact__Hard__Squelch.HitEnemy_Swipe__Hit_Body__Impact__Hard__Squelch")
    ;;[1 0 0.5859] Enemy Healthbar
    (bind _aswbp_enemy_health_bar (Utilities|Casting|CastToWBP_EnemyHealthBar (UserInterface|GetWidget (Variables|Default|GetHealtbar))))
    (Widget|SetVisibility _aswbp_enemy_health_bar "Visible")
    (Progress|SetPercent (Variables|/Game/Blueprints/UI/WBP_EnemyHealthBar.WBP_EnemyHealthBar_C|GetCurrentHealthbar _aswbp_enemy_health_bar) (/ (Variables|Stats|GetCurrent%20Health) (Variables|Stats|GetMaxHealth)))
    (Progress|SetPercent (Variables|/Game/Blueprints/UI/WBP_EnemyHealthBar.WBP_EnemyHealthBar_C|GetPrevHealthbar _aswbp_enemy_health_bar) (/ (Variables|Default|GetHealthBeforeDamage) (Variables|Stats|GetMaxHealth)))
    (Widget|SetVisibility (Variables|/Game/Blueprints/UI/WBP_EnemyHealthBar.WBP_EnemyHealthBar_C|GetDamagetake _aswbp_enemy_health_bar) "Visible")
    (Rendering|Components|TextRender|SetText (Variables|/Game/Blueprints/UI/WBP_EnemyHealthBar.WBP_EnemyHealthBar_C|GetDamageNumber _aswbp_enemy_health_bar) (Utilities|Text|ToText(Float) (Variables|Default|GetTakenDamage) "HalfToEven"))
    ;;[0.007812 1 0] Rest
    (Utilities|FlowControl|Delay 1.2)
    (Widget|SetVisibility (Variables|/Game/Blueprints/UI/WBP_EnemyHealthBar.WBP_EnemyHealthBar_C|GetDamagetake _aswbp_enemy_health_bar) "Collapsed")
    (Progress|SetPercent (Variables|/Game/Blueprints/UI/WBP_EnemyHealthBar.WBP_EnemyHealthBar_C|GetPrevHealthbar _aswbp_enemy_health_bar) (/ (Variables|Stats|GetCurrent%20Health) (Variables|Stats|GetMaxHealth)))
    (Variables|Default|SetTakenDamage 0.0)
    (Utilities|FlowControl|Delay 0.3)
    (if (not (Variables|Default|GetisStunned))
      (Variables|Default|SetisDamaged false)
      (Variables|Default|SetisAttacked false))))

(fn ConstructionScript)