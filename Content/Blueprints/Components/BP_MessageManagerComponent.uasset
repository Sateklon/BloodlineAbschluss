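; BP_MessageManagerComponent is a component that queues messages for display through a widget stack passed in by Setup.
; AddMessageToQueue appends a message only while the stack is valid, and calls ShowNextMessage when that message is the only one queued.
; ShowNextMessage is unfinished: it calls AddWidget on the stack without using the message, and nothing in the graph removes entries from the queue.
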(event Custom|Setup
  (params (Stack :type Common%20Activatable%20Widget%20Stack%20Object%20Reference))
  ;[1 0.2109 0] SetUp the Stack
  (Variables|Default|SetStack Stack))

(event Custom|AddMessageToQueue
  (params (Message :type STRUCT%20Message%20Structure%20%28by%20ref%29))
  ;[0 0.8828 1] ist der Stack valid ?
  (Utilities|IsValid (Variables|Default|GetStack)
    (:Is%20Valid
      ;[1 0 0.9375] Pack die Message in die Queue
      (Utilities|Array|Add (Variables|Default|GetMessageQueue) Message)
      (if (== (Utilities|Array|Length (Variables|Default|GetMessageQueue)) 1)
        (CallFunction|ShowNextMessage)))))

(event Custom|ShowNextMessage
  ;[0 1 0.1328] Zeig die Message .... [Weiter coden!!!]
  (Class|CommonActivatableWidgetContainerBase|AddWidget (Variables|Default|GetStack)))

(event EventBeginPlay)

(event EventTick
  (params (DeltaSeconds :type Float%20%28single-precision%29)))