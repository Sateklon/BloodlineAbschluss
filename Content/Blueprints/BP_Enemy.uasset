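; Enemy character for a 2D platformer that patrols, faces and attacks the player, awards souls on death and can respawn at its start position.
; A timer and ground/wall triggers turn it around, while Tick checks range and sets state flags for three randomized attack patterns with cooldown.
; Hits update a floating health bar and play feedback.
; Blood and Dark damage build timed stacks that trigger delayed bonus damage and stuns.
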(event OnComponentEndOverlap(AggroRange)
  (params (OverlappedComponent :type Primitive%20Component%20Object%20Reference) (OtherActor :type Actor%20Object%20Reference) (OtherComp :type Primitive%20Component%20Object%20Reference) (OtherBodyIndex :type Integer))
  ;[0.8281 1 0] Spieler verlässt die AggroRange
  (if (== OtherActor (Game|Player|GetPlayerPawn 0))
    (Variables|Default|SetChargeAttack true)
    (Variables|Stats|SetFirstAttack 0)
    (Variables|Default|SetisInAggroRange false)))

(event OnComponentBeginOverlap(AggroRange)
  (params (OverlappedComponent :type Primitive%20Component%20Object%20Reference) (OtherActor :type Actor%20Object%20Reference) (OtherComp :type Primitive%20Component%20Object%20Reference) (OtherBodyIndex :type Integer) (bFromSweep :type Boolean) (SweepResult :type Hit%20Result%20Structure%20%28by%20ref%29))
  ;[0 0.7422 1] Enemy vervolgt Spieler
  (if (not (Variables|Default|Getis%20Dead))
    ;;[1 0.04688 0] Ist der Spieler in Agro-Range ?
    (if (== OtherActor (Variables|Default|GetPlayer))
      (Variables|Default|SetisInAggroRange true)
      (Development|PrintString "is in Aggrorange")
      (if (and (not (Variables|Default|GetCantInterupt)) (not (Variables|Default|GetIsAttacking)))
        (bind _player (Variables|Default|GetPlayer)
          (:then
            ;;[0 0.4844 1] ist der Spieler rechts vom Gegner ?
            (Utilities|IsValid _player
              (:Is%20Valid
                (if (> (.x (Transformation|GetActorLocation _player)) (.x (Transformation|GetActorLocation)))
                  ;;[1 0 0.3281] Bewegt sich der Gegner schon nach rechts ?
                  (if (not (> (.x (Transformation|GetActorForwardVector)) 0.0))
                    (CallFunction|Turnaround))
                  (else
                    ;;[1 0.07031 0] Ist der Spieler links vom gegner ?
                    (bind _player_2 (Variables|Default|GetPlayer)
                      (:then
                        (if (< (.x (Transformation|GetActorLocation _player_2)) (.x (Transformation|GetActorLocation)))
                          ;;[0 1 0.625] bewegt sich der Gegner schon nach links ?
                          (if (not (< (.x (Transformation|GetActorForwardVector)) 0.0))
                            (CallFunction|Turnaround))))
                      (:else)))))))
          (:else))))))

(event OnComponentEndOverlap(Attackrange)
  (params (OverlappedComponent :type Primitive%20Component%20Object%20Reference) (OtherActor :type Actor%20Object%20Reference) (OtherComp :type Primitive%20Component%20Object%20Reference) (OtherBodyIndex :type Integer))
  ;[1 0.9141 0] Verlässt der Spieler die Attack range
  (if (== OtherActor (Game|Player|GetPlayerPawn 0))
    (Utilities|FlowControl|Delay 1.0)
    (Variables|Default|SetIsInAttackrange false)))

(event OnComponentEndOverlap(GroundCheck)
  (params (OverlappedComponent :type Primitive%20Component%20Object%20Reference) (OtherActor :type Actor%20Object%20Reference) (OtherComp :type Primitive%20Component%20Object%20Reference) (OtherBodyIndex :type Integer))
  ;[0 1 0.7422] GroundCheck
  (CallFunction|Turnaround))

(event OnComponentBeginOverlap(WalCheck)
  (params (OverlappedComponent :type Primitive%20Component%20Object%20Reference) (OtherActor :type Actor%20Object%20Reference) (OtherComp :type Primitive%20Component%20Object%20Reference) (OtherBodyIndex :type Integer) (bFromSweep :type Boolean) (SweepResult :type Hit%20Result%20Structure%20%28by%20ref%29))
  ;[1 0.09375 0] TileChecking
  (CallFunction|Turnaround))

(event Custom|KillEnemy
  ;[0 0.3906 1] Alles was bei Tot passieren soll
  (bind _asgm_plattformer (Utilities|Casting|CastToGM_Plattformer (Game|GetGameMode)))
  (Default|UpdateSouls _asgm_plattformer (Variables|Stats|GetSeelenwert))
  ;;[0.3828 1 0] für Achievment
  (Default|FirstEnemyKilled _asgm_plattformer)
  (Variables|Default|SetisAttacked false)
  (Variables|Default|SetIsAttacking false)
  (Variables|Default|SetisStunned false)
  (Collision|SetCollisionEnabled (Variables|Collision|GetCapsuleComponent) "NoCollision")
  ;[1 0 0.3516] Mach die Healthbar aus
  (bind _aswbp_enemy_health_bar (Utilities|Casting|CastToWBP_EnemyHealthBar (UserInterface|GetWidget (Variables|Default|GetHealthbar))))
  (Widget|SetVisibility _aswbp_enemy_health_bar "Collapsed")
  ;[0 0.3906 1] mach BloodDing aus, für den Fall das sie noch an ist
  (Variables|Damagetypes|SetBloodStacks -1)
  (Rendering|SetVisibility (Variables|Default|GetBloodDamageSprite) false false)
  (Rendering|SetVisibility (Variables|Default|GetDropShadow) false false))

(event Custom|BloodDamage
  ;[1 0.6094 0] BloodDamage
  ;;[1 0 0.8203] Wird schon Blutschaden gemacht ?
  (Development|PrintString "BloodDamage")
  (if (and (not (Variables|Damagetypes|GetisBloodmakingDamage)) (not (Variables|Default|Getis%20Dead)))
    ;;[0 0.6016 1] Blood an machen
    (Rendering|SetVisibility (Variables|Default|GetBloodDamageSprite) true false)
    (Utilities|Time|SetTimerbyEvent (delegate Custom|BloodCooldown) 3.0)
    (Utilities|FlowControl|Sequence
      (:then_0
        ;;[0.5234 1 0] Zähl die Stacks hoch
        (bind _output_get (Variables|Damagetypes|SetBloodStacks (+ (Variables|Damagetypes|GetBloodStacks) 1)))
        (if (>= _output_get 2)
          (Variables|Damagetypes|SetisBloodmakingDamage true)))
      (:then_1
        ;;[0.6875 0 1] Stack anzeigen
        (Rendering|Components|Sprite|SetSprite (Variables|Default|GetBloodDamageSprite) (Utilities|Array|Get(acopy) (Variables|Damagetypes|GetBloodStackSprites) (Variables|Damagetypes|GetBloodStacks))))
      (:then_2
        ;;[0.2422 0 1] nocjhmal checken ob alle stacks da sind
        (if (Variables|Damagetypes|GetisBloodmakingDamage)
          ;;[0 0.3672 1] Der eigentliche Blutschaden
          (Utilities|FlowControl|Delay 2.0)
          (if (> (Variables|Stats|GetHealth) 0.0)
            (Game|Damage|ApplyDamage self (Variables|/Game/Blueprints/GM_Plattformer.GM_Plattformer_C|GetCurrentBloodDamage (Variables|Default|GetGameManager)) 0 0 "/Game/Blueprints/Data/BP_DamageBlood.BP_DamageBlood_C")
            (CallFunction|EnemyStuning)
            (Class|FMODBlueprintStatics|PlayEvent2D "/Game/FMOD/Events/BloodDamage_ES_Intestines_Remove_2_-_SFX_Producer.BloodDamage_ES_Intestines_Remove_2_-_SFX_Producer")
            (Utilities|FlowControl|Delay 1.0)
            (Variables|Damagetypes|SetBloodStacks -1)
            (Variables|Damagetypes|SetisBloodmakingDamage false)
            (Rendering|SetVisibility (Variables|Default|GetBloodDamageSprite) false false)))))))

(event Custom|FindAllotherEnemys
  ;[1 0.4453 0] Find all other Enemys
  (Actor|GetAllActorsOfClass "BP_Enemy_C"))

(event Custom|Attack01Over
  ;[1 0 0.4687] Start der Attacke
  (Variables|Default|SetIsAttacking false)
  (Utilities|FlowControl|Sequence
    (:then_0
      (CallFunction|TurnAfterAttack)
      ;;[0 0.8594 1] AttackCooldown
      (Utilities|FlowControl|Delay (Variables|Stats|GetAttackSpeed))
      (Variables|Default|SetIsOnEnemyAttackCooldown false)
      (Utilities|FlowControl|DoOnce false) ; enters at Reset
    )
    (:then_1
      (Variables|Default|SetCantInterupt false))))

(event Custom|BloodCooldown
  ;[1 0.6094 0] BloodDamage
  ;;[0 0.6016 1] Blood an machen
  (Rendering|SetVisibility (Variables|Default|GetBloodDamageSprite) false false)
  (Variables|Damagetypes|SetBloodStacks -1))

(event Custom|EnemyTimer
  ;[1 0 0.3047] Enemy Timer für Patrulie
  (Utilities|FlowControl|Delay (Variables|Default|GetPatroulieZeit))
  (if (and (and (AI|Components|NavMovement|IsMovingonGround (Variables|Character|GetCharacterMovement)) (not (Math|Float|NearlyEqual(Float) (.x (Transformation|GetVelocity)) 0.0 0.001))) (and (not (Variables|Default|GetIsInAttackrange)) (not (Variables|Default|GetisInAggroRange))))
    (Utilities|FlowControl|DoOnce false :!label _label
      (:Completed
        (CallFunction|Turnaround)
        (Utilities|FlowControl|Delay 1.0)
        (Utilities|FlowControl|Sequence
          (:then_0
            (goto _label Reset))
          (:then_1
            (CallFunction|EnemyTimer)))))
    (else
      (CallFunction|EnemyTimer))))

(event Custom|EnemyStuning
  ;[1 0.3516 0] Enemy Stunning
  (if (Variables|Default|GetcanBeStunned)
    (Variables|Default|SetisStunned true)))

(event Custom|DarkDamage
  ;[0.8984 0 1] DarkDamage
  ;;[1 0.4922 0] Wird Dark Damage gemacht ?
  (if (== (not (Variables|Damagetypes|GetIsDarkDamageMaking)) (not (Variables|Default|Getis%20Dead)))
    ;;[0.4531 1 0] InputTimer
    (Rendering|SetVisibility (Variables|Default|GetDarkDamageSprite) true false)
    (Utilities|Time|SetTimerbyEvent (delegate Custom|DarkInpurCooldown) 3.0)
    (Utilities|FlowControl|Sequence
      (:then_0
        ;;[0 0.6016 1] Stackshochzählen
        (bind _output_get (Variables|Damagetypes|SetDarkStacks (+ (Variables|Damagetypes|GetDarkStacks) 1)))
        (if (>= _output_get 2)
          (Variables|Damagetypes|SetIsDarkDamageMaking true)))
      (:then_1
        ;;[0 0.3906 1] Sprite zeigen
        (Sprite|SetFlipbook (Variables|Default|GetDarkDamageSprite) (Utilities|Array|Get(acopy) (Variables|Damagetypes|GetDarkDamageSprites) (Variables|Damagetypes|GetDarkStacks))))
      (:then_2
        (if (Variables|Damagetypes|GetIsDarkDamageMaking)
          (Utilities|FlowControl|Delay 1.0)
          (if (> (Variables|Stats|GetHealth) 0.0)
            (if (not (Variables|Damagetypes|GetIsDarkDamageCooldown))
              (Development|PrintString "BurnSpriteFlipbook")
              (Development|PrintString "PlayFMODEvent")
              (Variables|Damagetypes|SetDarkStacks -1)
              (if (< (Variables|Damagetypes|GetDarkBurnStacks) 5) :!label _label
                (Game|Damage|ApplyDamage self (Variables|/Game/Blueprints/GM_Plattformer.GM_Plattformer_C|GetCurrentDarkDamage (Variables|Default|GetGameManager)) 0 0 "/Game/Blueprints/Data/BP_DamageDark.BP_DamageDark_C")
                (CallFunction|EnemyStuning)
                (Variables|Damagetypes|SetDarkBurnStacks (+ (Variables|Damagetypes|GetDarkBurnStacks) 1))
                (Utilities|FlowControl|Delay 0.2)
                (goto _label)
                (else
                  (Variables|Damagetypes|SetDarkBurnStacks 0)
                  (Utilities|FlowControl|Delay 0.2)
                  (Variables|Damagetypes|SetDarkStacks -1)
                  (Variables|Damagetypes|SetIsDarkDamageMaking false)
                  (Rendering|SetVisibility (Variables|Default|GetDarkDamageSprite) false false))))))))))

(event Custom|DarkInpurCooldown
  ;[0.8984 0 1] DarkDamage
  ;;[0.4531 1 0] InputTimer
  (Rendering|SetVisibility (Variables|Default|GetDarkDamageSprite) false false)
  (Variables|Damagetypes|SetDarkStacks -1))

(event Custom|Turn%20after%20Attack
  ;[1 0 0.375] TurnAfterAttack
  (if (Variables|Default|GetIsInAttackrange)
    ;[0 0.7422 1] Enemy vervolgt Spieler
    ;;[0 0.4844 1] ist der Spieler rechts vom Gegner ?
    (Utilities|IsValid (stale OnComponentBeginOverlap(AggroRange) _player)
      (:Is%20Valid
        (if (> (.x (Transformation|GetActorLocation (stale OnComponentBeginOverlap(AggroRange) _player))) (.x (Transformation|GetActorLocation)))
          ;;[1 0 0.3281] Bewegt sich der Gegner schon nach rechts ?
          (if (not (> (.x (Transformation|GetActorForwardVector)) 0.0))
            (CallFunction|Turnaround))
          (else
            ;;[1 0.07031 0] Ist der Spieler links vom gegner ?
            (bind _player (Variables|Default|GetPlayer)
              (:then
                (if (< (.x (Transformation|GetActorLocation _player)) (.x (Transformation|GetActorLocation)))
                  ;;[0 1 0.625] bewegt sich der Gegner schon nach links ?
                  (if (not (< (.x (Transformation|GetActorForwardVector)) 0.0))
                    (CallFunction|Turnaround))))
              (:else))))))))

(event Custom|TurnCheck
  (if (Variables|Default|GetisInAggroRange)
    ;[0 0.7422 1] Enemy vervolgt Spieler
    (if (and (not (Variables|Default|GetCantInterupt)) (not (Variables|Default|GetIsAttacking)))
      (bind _player (Variables|Default|GetPlayer)
        (:then
          ;;[0 0.4844 1] ist der Spieler rechts vom Gegner ?
          (Utilities|IsValid _player
            (:Is%20Valid
              (if (> (.x (Transformation|GetActorLocation _player)) (.x (Transformation|GetActorLocation)))
                ;;[1 0 0.3281] Bewegt sich der Gegner schon nach rechts ?
                (if (not (> (.x (Transformation|GetActorForwardVector)) 0.0))
                  (CallFunction|Turnaround))
                (else
                  ;;[1 0.07031 0] Ist der Spieler links vom gegner ?
                  (bind _player_2 (Variables|Default|GetPlayer)
                    (:then
                      (if (< (.x (Transformation|GetActorLocation _player_2)) (.x (Transformation|GetActorLocation)))
                        ;;[0 1 0.625] bewegt sich der Gegner schon nach links ?
                        (if (not (< (.x (Transformation|GetActorForwardVector)) 0.0))
                          (CallFunction|Turnaround))))
                    (:else)))))))
        (:else)))))

(event Custom|Attack01
  ;[0.9219 0 1] Attacks
  (for _array_element (Collision|GetOverlappingActors (Variables|Default|GetAttack01Collision) 0 :!class /Script/Engine.PrimitiveComponent)
    (if (!= _array_element self)
      (Game|Damage|ApplyDamage _array_element (Variables|Stats|GetBaseDamage) 0 self))))

(event Custom|Get%20Tilemap
  ;[0 1 0.08594] Get Tilemap
)

(event Custom|AttackCheck
  ;[1 0 0.8672] Ist der Player in der AttackRange ?
  (if (Collision|IsOverlappingActor (Variables|Default|GetAttackrange) (Game|Player|GetPlayerPawn 0) :!class /Script/Engine.PrimitiveComponent)
    (Utilities|FlowControl|Sequence
      (:then_0
        ;[1 0 0.7031] ChargeLogik
        (Variables|Default|SetIsInAttackrange true)
        (if (not (Variables|Default|GetIsAttacking))
          (if (not (Variables|Default|GetIsOnEnemyAttackCooldown))
            (Utilities|FlowControl|Delay 0.2)
            (if (Variables|Default|GetChargingEnemy)
              (Variables|Default|SetChargeAttack true))
            ;[1 0 0.4687] Start der Attacke
            (Utilities|FlowControl|DoOnce false
              (:Completed
                ;[1 0.75 0] Mit welcher Attacke soll gestartet werden ?
                (switch int (Variables|Stats|GetFirstAttack)
                  (:0
                    ;[1 0.8906 0] Attackdurchführung
                    ;;[0 1 0.9297] Attack01
                    (if (Variables|Default|GetChargeAttack)
                      (Utilities|FlowControl|Delay 0.0)
                      (else
                        (Utilities|FlowControl|Delay 1.0)))
                    (Variables|Default|SetCantInterupt true)
                    (Variables|Default|SetIsAttacking true)
                    (Variables|Default|SetIsOnEnemyAttackCooldown true)
                    (bind _output_get (Variables|Default|SetAttackNumber 0))
                    (Development|PrintString (Utilities|String|ToString(Integer) _output_get))
                    ;;[1 0 0.2578] Nächster Angriff ist random
                    (Variables|Stats|SetFirstAttack (Math|Random|RandomInteger 3)))
                  (:1
                    ;;[0 1 0.0625] Attack02
                    (Utilities|FlowControl|Delay 1.0)
                    (Variables|Default|SetCantInterupt true)
                    (Variables|Default|SetIsAttacking true)
                    (Variables|Default|SetIsOnEnemyAttackCooldown true)
                    (bind _output_get_2 (Variables|Default|SetAttackNumber 1))
                    (Development|PrintString (Utilities|String|ToString(Integer) _output_get_2))
                    (Variables|Stats|SetFirstAttack (Math|Random|RandomInteger 3)))
                  (:2
                    ;;[1 0 0.1172] Attack Kombi (erst 01, dann 02)
                    (Utilities|FlowControl|Delay 1.0)
                    (Variables|Default|SetCantInterupt true)
                    (Variables|Default|SetIsAttacking true)
                    (Variables|Default|SetIsOnEnemyAttackCooldown true)
                    (bind _output_get_3 (Variables|Default|SetAttackNumber 2))
                    (Development|PrintString (Utilities|String|ToString(Integer) _output_get_3))
                    (Variables|Stats|SetFirstAttack (Math|Random|RandomInteger 3))))))))))))

(event Custom|Attack02
  ;[0.9219 0 1] Attacks
  (for _array_element (Collision|GetOverlappingActors (Variables|Default|GetAttack02Collision) 0 :!class /Script/Engine.PrimitiveComponent)
    (if (!= _array_element self)
      (Game|Damage|ApplyDamage _array_element (Variables|Stats|GetBaseDamage) 0 self))))

(event Custom|Turnaround
  ;[1 0.8438 0] Turn arround
  (Transformation|SetActorRotation (Math|Rotator|CombineRotators (Transformation|GetActorRotation) "0.000000,180.000000,0.000000")))

(event Custom|Attack02Over
  ;[1 0 0.4687] Start der Attacke
  (Variables|Default|SetIsAttacking false)
  (Utilities|FlowControl|Sequence
    (:then_0
      (CallFunction|TurnAfterAttack)
      ;;[0 0.8594 1] AttackCooldown
      (Utilities|FlowControl|Delay (Variables|Stats|GetAttackSpeed))
      (Variables|Default|SetIsOnEnemyAttackCooldown false)
      (Utilities|FlowControl|DoOnce false) ; enters at Reset
    )
    (:then_1
      (Variables|Default|SetCantInterupt false))))

(event Custom|MoveForward
  ;[0.1484 1 0] KIMovement
  (if (not (Variables|Default|GetIsInAttackrange))
    (if (not (Variables|Default|GetCantInterupt))
      (if (and (and (and (not (Variables|Default|GetisStunned)) (not (Variables|Default|Getis%20Dead))) (not (Variables|Default|GetIsAttacking))) (not (Variables|Default|GetIsOnEnemyAttackCooldown)))
        (Pawn|Input|AddMovementInput (Transformation|GetActorForwardVector) 1.0 false)))))

(event Custom|EnemySetup
  ;[0.8516 0 1] Setup
  (Variables|Stats|SetHealth (Variables|Stats|GetMaxHealth))
  (Variables|Default|SetStartposition (Transformation|GetActorLocation))
  ;[0 0.6016 1] Blood aus machen
  (Rendering|SetVisibility (Variables|Default|GetBloodDamageSprite) false false))

(event EventRespawn
  ;[1 0 0.8437] Respawn
  (Variables|Damagetypes|SetBloodStacks -1)
  (Variables|Stats|SetHealth (Variables|Stats|GetMaxHealth))
  (Transformation|SetActorLocation (Variables|Default|GetStartposition) false false)
  (Variables|Default|SetisDamageing false)
  (Variables|Default|Setis%20Dead false)
  (Variables|Default|SetisStunned false)
  (Variables|Damagetypes|SetIsDarkDamageMaking false)
  (Variables|Default|SetIsOnEnemyAttackCooldown false)
  (Variables|Default|SetCantInterupt false)
  (Variables|Default|SetIsInAttackrange false)
  (Utilities|FlowControl|Delay 0.2)
  (Collision|SetCollisionEnabled (Variables|Collision|GetCapsuleComponent) "QueryAndPhysics")
  ;[1 0 0.3516] Mach die Healthbar aus
  (bind _aswbp_enemy_health_bar (Utilities|Casting|CastToWBP_EnemyHealthBar (UserInterface|GetWidget (Variables|Default|GetHealthbar)))
    (:then
      (Widget|SetVisibility _aswbp_enemy_health_bar "Collapsed"))
    (:CastFailed
      _))
  ;[0 1 0.8828] AttackReset
  (CallFunction|Attack01Over)
  (bind _asbp_player (Utilities|Casting|CastToBP_Player (Game|Player|GetPlayerPawn 0)))
  (Variables|Default|SetPlayer _asbp_player)
  (Rendering|SetVisibility (Variables|Default|GetDropShadow) true false))

(event EventBeginPlay
  ;[0.5469 1 0] Beginn
  (CallFunction|EnemySetup)
  (CallFunction|FindAllotherEnemys)
  ;[0.05469 0 1] GetGameManager
  (bind _asgm_plattformer (Utilities|Casting|CastToGM_Plattformer (Game|GetGameMode)))
  (Variables|Default|SetGameManager _asgm_plattformer)
  (CallFunction|EnemyTimer)
  ;[1 0 0.375] Get Player
  (bind _asbp_player (Utilities|Casting|CastToBP_Player (Game|Player|GetPlayerPawn 0)))
  (Variables|Default|SetPlayer _asbp_player))

(event Game|Damage|EventAnyDamage
  (params (Damage :type Float%20%28single-precision%29) (DamageType :type Damage%20Type%20Object%20Reference) (InstigatedBy :type Controller%20Object%20Reference) (DamageCauser :type Actor%20Object%20Reference))
  ;[0 1 0.01562] SetupDamageType (Bisher NUR Blooddamage)
  ;;[1 0.9375 0] Player finden
  (bind _asbp_player (Utilities|Casting|CastToBP_Player (Game|Player|GetPlayerPawn 0)))
  (Variables|Default|SetPlayer _asbp_player)
  (if (and (not (== DamageCauser self)) (== (Utilities|GetClass DamageType) (Variables|Stats|GetWoundableDamagetype)))
    (if (== (Variables|Stats|GetWoundableDamagetype) (Variables|Damagetypes|GetBloodDamageClass))
      (CallFunction|BloodDamage)
      (elif (== (Variables|Stats|GetWoundableDamagetype) (Variables|Damagetypes|GetDarkDamageClass))
        (CallFunction|DarkDamage))))
  ;[1 0 0.07031] HP verlieren
  (if (not (Variables|Default|Getis%20Dead))
    (Variables|Default|SetisAttacked true)
    (Variables|Default|SetHealthBeforeDamage (Variables|Stats|GetHealth))
    (Variables|Default|SetTakenDamage (+ (Variables|Default|GetTakenDamage) Damage))
    (bind _output_get (Variables|Stats|SetHealth (- (Variables|Stats|GetHealth) Damage)))
    (Camera|PlayWorldCameraShake "/Game/Blueprints/BP_CameraShake_Damage.BP_CameraShake_Damage_C" (Transformation|GetWorldLocation (Variables|/Game/Blueprints/BP_Player.BP_Player_C|GetCamera (Variables|Default|GetPlayer))) 0.0 2e+02)
    (Game|Feedback|ClientPlayForceFeedback (Game|GetPlayerController 0) "/Game/Blueprints/ControllerVibration/PlayerAttackHitVoibration.PlayerAttackHitVoibration" "None" false false false)
    (Class|FMODBlueprintStatics|PlayEvent2D "/Game/FMOD/Events/HitEnemy_Swipe__Hit_Body__Impact__Hard__Squelch.HitEnemy_Swipe__Hit_Body__Impact__Hard__Squelch")
    ;[0.4062 1 0] Absicherung
    (if (<= _output_get 0.0)
      (Variables|Default|Setis%20Dead true)
      (else
        (Variables|Default|SetisDamageing true)))
    ;[1 0 0.5859] Enemy Healthbar
    (bind _aswbp_enemy_health_bar (Utilities|Casting|CastToWBP_EnemyHealthBar (UserInterface|GetWidget (Variables|Default|GetHealthbar))))
    (Widget|SetVisibility _aswbp_enemy_health_bar "Visible")
    (Progress|SetPercent (Variables|/Game/Blueprints/UI/WBP_EnemyHealthBar.WBP_EnemyHealthBar_C|GetCurrentHealthbar _aswbp_enemy_health_bar) (/ (Variables|Stats|GetHealth) (Variables|Stats|GetMaxHealth)))
    (Progress|SetPercent (Variables|/Game/Blueprints/UI/WBP_EnemyHealthBar.WBP_EnemyHealthBar_C|GetPrevHealthbar _aswbp_enemy_health_bar) (/ (Variables|Default|GetHealthBeforeDamage) (Variables|Stats|GetMaxHealth)))
    (Widget|SetVisibility (Variables|/Game/Blueprints/UI/WBP_EnemyHealthBar.WBP_EnemyHealthBar_C|GetDamagetake _aswbp_enemy_health_bar) "Visible")
    (Rendering|Components|TextRender|SetText (Variables|/Game/Blueprints/UI/WBP_EnemyHealthBar.WBP_EnemyHealthBar_C|GetDamageNumber _aswbp_enemy_health_bar) (Utilities|Text|ToText(Float) (Variables|Default|GetTakenDamage) "HalfToEven"))
    ;[0 0.6719 1] Stoppe den gegner
    (Pawn|Input|AddMovementInput "1.000000,0.000000,0.000000" 0.0 false)
    ;[0.8281 1 0] HelthbarUpdate
    (Utilities|FlowControl|Delay 1.0)
    (Widget|SetVisibility (Variables|/Game/Blueprints/UI/WBP_EnemyHealthBar.WBP_EnemyHealthBar_C|GetDamagetake _aswbp_enemy_health_bar) "Collapsed")
    (Progress|SetPercent (Variables|/Game/Blueprints/UI/WBP_EnemyHealthBar.WBP_EnemyHealthBar_C|GetPrevHealthbar _aswbp_enemy_health_bar) (/ (Variables|Stats|GetHealth) (Variables|Stats|GetMaxHealth)))
    ;[1 0.3281 0] Absicherung
    (Variables|Default|SetTakenDamage 0.0)
    (Utilities|FlowControl|Sequence
      (:then_0
        (Utilities|FlowControl|Delay 0.2)
        (CallFunction|Attack01Over))
      (:then_1
        (if (not (Variables|Default|GetisStunned))
          (Variables|Default|SetisDamageing false)
          (Variables|Default|SetisAttacked false))))))

(event EventTick
  (params (DeltaSeconds :type Float%20%28single-precision%29))
  ;[1 0 0.8672] TICK
  (CallFunction|AttackCheck)
  (CallFunction|GetTilemap)
  (CallFunction|TurnCheck))

(fn ConstructionScript)

(fn UpdateAnim)

(fn RestartAnim
  ;[0.5469 0 1] Loop wieder
  (Sprite|SetFlipbook (Variables|Default|GetSprite))
  (Components|Timeline|SetLooping (Variables|Default|GetSprite) true)
  ;[0.2891 0 1] Start Anim
  (if (not (Audio|Components|Audio|IsPlaying (Variables|Default|GetSprite)))
    (Audio|Components|Audio|Play (Variables|Default|GetSprite))))

(fn GetEnemyStats
  (return (Variables|Default|GetEnemyType)))