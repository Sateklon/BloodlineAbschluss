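; BP_FakeWall is a sprite-based fake wall that disappears when it takes any damage.
; The first hit, gated by DoOnce, makes the render component movable and plays a 2D metallic impact sound.
; A timeline then fades the wall sprite and its Hint sprite to transparent by lerping their alpha, and destroys the actor when finished.
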(event EventBeginPlay)

(event Game|Damage|EventAnyDamage
  (params (Damage :type Float%20%28single-precision%29) (DamageType :type Damage%20Type%20Object%20Reference) (InstigatedBy :type Controller%20Object%20Reference) (DamageCauser :type Actor%20Object%20Reference))
  (bind _hint (Variables|Default|GetHint))
  (bind _rendercomponent (Variables|Default|GetRenderComponent))
  (bind _spritecolor (Variables|/Script/Paper2D.PaperSpriteComponent|GetSpriteColor _hint))
  (bind _spritecolor_2 (Variables|/Script/Paper2D.PaperSpriteComponent|GetSpriteColor _rendercomponent))
  ;[0.8984 1 0] FakeWall verschwindibus
  (Utilities|FlowControl|DoOnce false
    (:Completed
      (Transformation|SetMobility (Variables|Default|GetRenderComponent) "Movable")
      (Class|FMODBlueprintStatics|PlayEvent2D "/Game/FMOD/Events/FakeWall_ES_Hit_Metallic_Impact_5_-_SFX_Producer.FakeWall_ES_Hit_Metallic_Impact_5_-_SFX_Producer")
      (bind _alpha (Timeline|Timeline PlayFromStart)
        (:Update
          (Utilities|FlowControl|Sequence
            (:then_0
              (Sprite|SetSpriteColor _hint (Utilities|Struct|MakeLinearColor (.r _spritecolor) (.g _spritecolor) (.b _spritecolor) (Math|Float|Lerp 0.5 0.0 _alpha))))
            (:then_1
              (Sprite|SetSpriteColor _rendercomponent (Utilities|Struct|MakeLinearColor (.r _spritecolor_2) (.g _spritecolor_2) (.b _spritecolor_2) (Math|Float|Lerp 1.0 0.0 _alpha))))))
        (:Finished
          (Actor|DestroyActor))))))

(event EventTick
  (params (DeltaSeconds :type Float%20%28single-precision%29)))

(event Collision|EventActorBeginOverlap
  (params (OtherActor :type Actor%20Object%20Reference)))

(fn ConstructionScript)