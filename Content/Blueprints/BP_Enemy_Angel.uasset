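; Flying angel enemy for a 2D platformer that follows a spline, optionally looping, and shoots arrows at the player.
; Tick moves the flipbook and aims; in aggro range a DoOnce plays the shooting animation, re-armed after ShootArrow's AttackSpeed delay.
; Damage drives health bar and hit feedback, and death awards souls through GM_Plattformer.
; Dark damage stacks into a self-applied burst of ticks; blood damage is an empty stub.
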(event OnComponentBeginOverlap(AggroRange)
  (params (OverlappedComponent :type Primitive%20Component%20Object%20Reference) (OtherActor :type Actor%20Object%20Reference) (OtherComp :type Primitive%20Component%20Object%20Reference) (OtherBodyIndex :type Integer) (bFromSweep :type Boolean) (SweepResult :type Hit%20Result%20Structure%20%28by%20ref%29))
  ;[0.8281 1 0] IsInAggroRange
  (if (== OtherActor (Variables|Default|GetPlayer))
    (Variables|Default|SetisInAggroRange true)))

(event OnComponentEndOverlap(AggroRange)
  (params (OverlappedComponent :type Primitive%20Component%20Object%20Reference) (OtherActor :type Actor%20Object%20Reference) (OtherComp :type Primitive%20Component%20Object%20Reference) (OtherBodyIndex :type Integer))
  ;[0.8047 1 0] IsNOTInAggrorange
  (if (== OtherActor (Variables|Default|GetPlayer))
    (Variables|Default|SetisInAggroRange false)))

(event Custom|Shoot
  ;[0.4531 1 0] Shooting
  (if (and (Variables|Default|GetisInAggroRange) (not (Variables|Default|GetisDead)))
    (Utilities|FlowControl|DoOnce false
      (:Completed
        ;;[0.3359 1 0] Animation
        (Class|PaperZDAnimInstance|JumptoNode (Variables|/Script/PaperZD.PaperZDAnimationComponent|GetAnimInstance (Variables|Default|GetAnimation%20Component)) "Shooting" "None")))))

(event Custom|Tracking%20Player
  ;[0.6641 1 0] PlayerTracking
  ;;[0 0.5547 1] Schussrichtung
  (bind _player (Variables|Default|GetPlayer)
    (:then
      (Transformation|SetRelativeRotation (Variables|Default|GetArrow) (Math|Rotator|MakeRotator 0.0 (.pitch (Math|Rotator|FindLookatRotation (Transformation|GetWorldLocation (Variables|Default|GetArrow)) (Transformation|GetActorLocation _player))) 0.0) false false))
    (:else
      (bind _asbp_player (Utilities|Casting|CastToBP_Player (Game|Player|GetPlayerPawn 0)))
      (Variables|Default|SetPlayer _asbp_player))))

(event Custom|DarkInpurCooldown
  ;[0.5469 1 0] Dark Damage
  (Rendering|SetVisibility (Variables|Default|GetDarkDamageFlipbook) false false)
  (Variables|Default|SetDarkStacks -1))

(event Custom|Look%20at%20Player
  ;[0.6641 1 0] PlayerTracking
  ;;[0 1 0.4609] Rechts vom Gegner ?
  (bind _player (Variables|Default|GetPlayer)
    (:then
      _)
    (:else
      (bind _asbp_player (Utilities|Casting|CastToBP_Player (Game|Player|GetPlayerPawn 0)))
      (Variables|Default|SetPlayer _asbp_player)))
  (if (> (.x (Transformation|GetActorLocation _player)) (.x (Transformation|GetWorldLocation (Variables|Default|GetAngelFlipbook))))
    ;;[0 1 0.6719] Bewegt sich schon nach rechts ?
    (if (not (> (.x (Transformation|GetActorLocation (Variables|Default|GetPlayer))) (.x (Transformation|GetWorldLocation (Variables|Default|GetAngelFlipbook)))))
      (CallFunction|Turnaround))
    (else
      ;;[0.9922 1 0] Links vom Gegner ?
      (if (< (.x (Transformation|GetActorLocation (Variables|Default|GetPlayer))) (.x (Transformation|GetWorldLocation (Variables|Default|GetAngelFlipbook))))
        ;;[0 1 0.625] bewegt sich der Gegner schon nach links ?
        (if (< (.x (Transformation|GetActorLocation (Variables|Default|GetPlayer))) (.x (Transformation|GetWorldLocation (Variables|Default|GetAngelFlipbook))))
          (CallFunction|Turnaround))))))

(event Custom|KillEnemy
  ;[0.6875 1 0] Angel Die
  (bind _aswbp_enemy_health_bar (Utilities|Casting|CastToWBP_EnemyHealthBar (UserInterface|GetWidget (Variables|Default|GetHealtbar))))
  (Widget|SetVisibility _aswbp_enemy_health_bar "Collapsed")
  (Rendering|SetVisibility (Variables|Default|GetHealtbar) false false)
  (bind _asgm_plattformer (Utilities|Casting|CastToGM_Plattformer (Game|GetGameMode)))
  (Default|UpdateSouls _asgm_plattformer (Variables|Stats|GetSoulvalue))
  ;;[0.5234 0 1] Absicherung
  (Variables|Default|SetisDead true))

(event Custom|ShootOver
  ;[0.4531 1 0] Shooting
  (Utilities|FlowControl|DoOnce false) ; enters at Reset
)

(event Custom|ShootArrow
  ;[0.4531 1 0] Shooting
  (bind _returnvalue (Game|SpawnActorfromClass "/Game/Blueprints/BP_AngelArrow.BP_AngelArrow_C" (Transformation|GetWorldTransform (Variables|Default|GetArrow)) "AlwaysSpawn" "MultiplyWithRoot" 0 0))
  (Utilities|IsValid _returnvalue
    (:Is%20Valid
      (Default|SetArrowDamage _returnvalue (Variables|Stats|GetDamage))
      (Utilities|FlowControl|Delay (Variables|Stats|GetAttackSpeed))
      (CallFunction|ShootOver))
    (:Is%20Not%20Valid
      (CallFunction|ShootOver))))

(event Custom|Turnaround
  ;[0 1 0.8828] Turn arround
  (Transformation|SetRelativeRotation (Variables|Default|GetAngelFlipbook) (Math|Rotator|CombineRotators (Transformation|GetActorRotation) "0.000000,180.000000,0.000000") false false))

(event Custom|BloodDamage)

(event Custom|DarkDamage
  ;[0.5469 1 0] Dark Damage
  (if (== (not (Variables|Default|GetIsDarkDamageMaking)) (not (Variables|Default|GetisDead)))
    (Rendering|SetVisibility (Variables|Default|GetDarkDamageFlipbook) true false)
    (Utilities|Time|SetTimerbyEvent (delegate Custom|DarkInpurCooldown) 3.0)
    (Utilities|FlowControl|Sequence
      (:then_0
        (bind _output_get (Variables|Default|SetDarkStacks (+ (Variables|Default|GetDarkStacks) 1)))
        (if (>= _output_get 2)
          (Variables|Default|SetIsDarkDamageMaking true)))
      (:then_1
        (Sprite|SetFlipbook (Variables|Default|GetDarkDamageFlipbook) (Utilities|Array|Get(acopy) (Variables|Default|GetDarkDamageSprites) (Variables|Default|GetDarkStacks))))
      (:then_2
        (if (Variables|Default|GetIsDarkDamageMaking)
          (Utilities|FlowControl|Delay 1.0)
          (if (> (Variables|Stats|GetCurrentHealth) 0.0)
            (if (not (Variables|Default|GetIsDarkDamageCooldown))
              (Development|PrintString "BurnSpriteFlipbook")
              (Development|PrintString "PlayFMODEvent")
              (Variables|Default|SetDarkStacks -1)
              (if (< (Variables|Default|GetDarkBurnStacks) 5) :!label _label
                (Game|Damage|ApplyDamage self (Variables|/Game/Blueprints/GM_Plattformer.GM_Plattformer_C|GetCurrentDarkDamage (Variables|Default|GetGameManager)) 0 0 "/Game/Blueprints/Data/BP_DamageDark.BP_DamageDark_C")
                (Variables|Default|SetDarkBurnStacks (+ (Variables|Default|GetDarkBurnStacks) 1))
                (Utilities|FlowControl|Delay 0.2)
                (goto _label)
                (else
                  (Variables|Default|SetDarkBurnStacks 0)
                  (Utilities|FlowControl|Delay 0.2)
                  (Variables|Default|SetDarkStacks -1)
                  (Variables|Default|SetIsDarkDamageMaking false)
                  (Rendering|SetVisibility (Variables|Default|GetDarkDamageFlipbook) false false))))))))))

(event EventRespawn
  ;[0 0.01562 1] Respawn
  (Variables|Stats|SetCurrentHealth (Variables|Stats|GetMaxHealth))
  (Variables|Default|SetisDead false)
  (bind _aswbp_enemy_health_bar (Utilities|Casting|CastToWBP_EnemyHealthBar (UserInterface|GetWidget (Variables|Default|GetHealtbar))))
  (Widget|SetVisibility _aswbp_enemy_health_bar "Collapsed")
  (Rendering|SetVisibility (Variables|Default|GetHealtbar) true false)
  (bind _asbp_player (Utilities|Casting|CastToBP_Player (Game|Player|GetPlayerPawn 0)))
  (Variables|Default|SetPlayer _asbp_player))

(event EventTick
  (params (DeltaSeconds :type Float%20%28single-precision%29))
  ;[0.7109 0 1] Das Angel-Movement entlang der Spline
  (if (not (Variables|Default|GetisDead))
    (Variables|Default|SetDistance%20Along%20Spline (+ (* DeltaSeconds (Variables|Stats|GetMove%20Speed)) (Variables|Default|GetDistance%20Along%20Spline)))
    (Transformation|SetRelativeTransform (Variables|Default|GetAngelFlipbook) (Math|Transform|MakeTransform (.location (Spline|GetTransformatDistanceAlongSpline (Variables|Default|GetSpline) (Variables|Default|GetDistance%20Along%20Spline) "Local" false)) "0, 0, 0" "1.000000,1.000000,1.000000") false false)
    (CallFunction|LookatPlayer)
    (CallFunction|TrackingPlayer)
    (CallFunction|Shoot)
    ;[0.6172 1 0] Looping
    (if (Variables|Essentiials|GetCanLoop)
      (if (> (Variables|Default|GetDistance%20Along%20Spline) (Spline|GetSplineLength (Variables|Default|GetSpline)))
        (Variables|Default|SetDistance%20Along%20Spline 0.0)))))

(event EventBeginPlay
  ;[0 1 0.8594] Beginn Play
  (bind _asbp_player (Utilities|Casting|CastToBP_Player (Game|Player|GetPlayerPawn 0)))
  (Variables|Default|SetPlayer _asbp_player)
  (Variables|Stats|SetCurrentHealth (Variables|Stats|GetMaxHealth))
  (bind _asgm_plattformer (Utilities|Casting|CastToGM_Plattformer (Game|GetGameMode)))
  (Variables|Default|SetGameManager _asgm_plattformer)
  ;[0 0.6016 1] Blood aus machen
  (Rendering|SetVisibility (Variables|Default|GetBloodDamageSprite) false false))

(event Game|Damage|EventAnyDamage
  (params (Damage :type Float%20%28single-precision%29) (DamageType :type Damage%20Type%20Object%20Reference) (InstigatedBy :type Controller%20Object%20Reference) (DamageCauser :type Actor%20Object%20Reference))
  ;[0 1 0.2266] Take Damage
  ;;[1 0.9375 0] Player finden
  (bind _asbp_player (Utilities|Casting|CastToBP_Player (Game|Player|GetPlayerPawn 0)))
  (Variables|Default|SetPlayer _asbp_player)
  (if (and (not (== DamageCauser self)) (== (Utilities|GetClass DamageType) (Variables|Default|GetWoundableDamagetype)))
    (if (== (Variables|Default|GetWoundableDamagetype) (Variables|Default|GetBloodDamageClass))
      (CallFunction|BloodDamage)
      (elif (== (Variables|Default|GetWoundableDamagetype) (Variables|Default|GetDarkDamageClass))
        (CallFunction|DarkDamage))))
  ;;[1 0.2109 0] DamageMathe
  (if (not (Variables|Default|GetisDead))
    (Variables|Default|SetHealth%20Before%20Damage (Variables|Stats|GetCurrentHealth))
    (Variables|Default|SetTakenDamage (+ (Variables|Default|GetTakenDamage) Damage))
    (bind _output_get (Variables|Stats|SetCurrentHealth (- (Variables|Stats|GetCurrentHealth) Damage)))
    ;;[0.9688 0 1] Absicherung
    (if (<= _output_get 0.0)
      (Variables|Default|SetisDead true)
      ;;[1 0 0.375] KILL
      (CallFunction|KillEnemy))
    ;;[0 1 0.625] Fancy Stuff
    (Camera|PlayWorldCameraShake "/Game/Blueprints/BP_CameraShake_Damage.BP_CameraShake_Damage_C" (Transformation|GetWorldLocation (Variables|/Game/Blueprints/BP_Player.BP_Player_C|GetCamera (Variables|Default|GetPlayer))) 0.0 2e+02)
    ;;;[0.3359 1 0] Animation
    (Class|PaperZDAnimInstance|JumptoNode (Variables|/Script/PaperZD.PaperZDAnimationComponent|GetAnimInstance (Variables|Default|GetAnimation%20Component)) "Damage" "None")
    (Game|Feedback|ClientPlayForceFeedback (Game|GetPlayerController 0) "/Game/Blueprints/ControllerVibration/PlayerAttackHitVoibration.PlayerAttackHitVoibration" "None" false false false)
    (Class|FMODBlueprintStatics|PlayEvent2D "/Game/FMOD/Events/HitEnemy_Swipe__Hit_Body__Impact__Hard__Squelch.HitEnemy_Swipe__Hit_Body__Impact__Hard__Squelch")
    ;;[1 0 0.5859] Enemy Healthbar
    (bind _aswbp_enemy_health_bar (Utilities|Casting|CastToWBP_EnemyHealthBar (UserInterface|GetWidget (Variables|Default|GetHealtbar))))
    (Widget|SetVisibility _aswbp_enemy_health_bar "Visible")
    (Progress|SetPercent (Variables|/Game/Blueprints/UI/WBP_EnemyHealthBar.WBP_EnemyHealthBar_C|GetCurrentHealthbar _aswbp_enemy_health_bar) (/ (Variables|Stats|GetCurrentHealth) (Variables|Stats|GetMaxHealth)))
    (Progress|SetPercent (Variables|/Game/Blueprints/UI/WBP_EnemyHealthBar.WBP_EnemyHealthBar_C|GetPrevHealthbar _aswbp_enemy_health_bar) (/ (Variables|Default|GetHealth%20Before%20Damage) (Variables|Stats|GetMaxHealth)))
    (Widget|SetVisibility (Variables|/Game/Blueprints/UI/WBP_EnemyHealthBar.WBP_EnemyHealthBar_C|GetDamagetake _aswbp_enemy_health_bar) "Visible")
    (Rendering|Components|TextRender|SetText (Variables|/Game/Blueprints/UI/WBP_EnemyHealthBar.WBP_EnemyHealthBar_C|GetDamageNumber _aswbp_enemy_health_bar) (Utilities|Text|ToText(Float) (Variables|Default|GetTakenDamage) "HalfToEven"))
    ;;[0.007812 1 0] Rest
    (Utilities|FlowControl|Delay 1.2)
    (Widget|SetVisibility (Variables|/Game/Blueprints/UI/WBP_EnemyHealthBar.WBP_EnemyHealthBar_C|GetDamagetake _aswbp_enemy_health_bar) "Collapsed")
    (Progress|SetPercent (Variables|/Game/Blueprints/UI/WBP_EnemyHealthBar.WBP_EnemyHealthBar_C|GetPrevHealthbar _aswbp_enemy_health_bar) (/ (Variables|Stats|GetCurrentHealth) (Variables|Stats|GetMaxHealth)))))

(fn ConstructionScript)