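; BP_CameraSpline is a camera spline actor that can register itself as the player's initial spline when play begins.
; On BeginPlay it caches the BP_Player pawn and waits briefly.
; If flagged as the first spline, it sets itself as the player's CameraSplineRef and GM_Plattformer's ActiveSpline, then passes itself to the game mode's RespawningSpline.
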(event EventBeginPlay
  (bind _asbp_player (Utilities|Casting|CastToBP_Player (Game|Player|GetPlayerPawn 0)))
  (Variables|Default|SetPlayer _asbp_player)
  (Utilities|FlowControl|Delay 0.2)
  (if (Variables|Default|GetIsFirstSpline)
    (Variables|/Game/Blueprints/BP_Player.BP_Player_C|SetCameraSplineRef (Variables|Default|GetPlayer) self)
    (bind _asgm_plattformer (Utilities|Casting|CastToGM_Plattformer (Game|GetGameMode)))
    (Variables|/Game/Blueprints/GM_Plattformer.GM_Plattformer_C|SetActiveSpline _asgm_plattformer self)
    (Default|RespawningSpline _asgm_plattformer self)))

(fn ConstructionScript)