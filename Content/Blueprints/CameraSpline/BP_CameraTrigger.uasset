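; Camera trigger for a platformer that switches the active camera spline when the player overlaps it, optionally starting a boss encounter.
; The switch is hidden behind a screen fade, with input disabled and the player's InterpSpeed temporarily zeroed.
; In boss areas, a timeline zooms out the orthographic camera, then activates whichever boss is assigned and animates the room barriers.
; Other areas reset the camera to the normal ortho width.
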(event Custom|CameraWithChange
  ;[0.2656 0 1] Ist es ne BossArea
  (if (Variables|NurRelevantBeiBossen|GetIsBossArea)
    (Input|DisableInput (Variables|Default|GetPlayer) (Game|GetPlayerController 0))
    ;[0.5703 1 0] ZoomOut
    (bind _alpha (Timeline|ZoomOut PlayFromStart)
      (:Update
        (Class|CameraComponent|SetOrthoWidth (Variables|/Game/Blueprints/BP_Player.BP_Player_C|GetCamera (Variables|Default|GetPlayer)) (Math|Float|Lerp (Variables|Default|GetCurrentOrthoWidth) 3e+03 _alpha)))
      (:Finished
        (Utilities|FlowControl|Sequence
          (:then_0
            ;;[1 0.5391 0] Boss1 Aktivieren
            (bind _waldschradtboss (Variables|NurRelevantBeiBossen|GetWaldschradtboss)
              (:then
                (Default|ActivateBoss _waldschradtboss)
                ;;[1 0.3984 0] Boss Absperrungen
                (for _array_element (Variables|NurRelevantBeiBossen|GetRaumAbsperrung) :!label _label
                  (Utilities|IsValid _array_element
                    (:Is%20Valid
                      (bind _asbp_boss_01absperrung (Utilities|Casting|CastToBP_Boss01Absperrung _array_element))
                      (Default|PlayAnim _asbp_boss_01absperrung)))))
              (:else)))
          (:then_1
            ;;[0 0.7422 1] Boss02 Aktivieren
            (bind _endboss (Variables|NurRelevantBeiBossen|GetEndboss)
              (:then
                (Default|ActivateBOSS _endboss)
                (goto _label))
              (:else)))
          (:then_2
            (Input|EnableInput (Variables|Default|GetPlayer) (Game|GetPlayerController 0))))))
    (else
      ;[1 0 0.6094] Normale CamEinstellung
      (Class|CameraComponent|SetOrthoWidth (Variables|/Game/Blueprints/BP_Player.BP_Player_C|GetCamera (Variables|Default|GetPlayer)) 2.3e+03))))

(event Custom|Get%20CameraWith
  ;[1 0.4922 0] Get Otho with
  (Variables|Default|SetCurrentOrthoWidth (Variables|/Script/Engine.CameraComponent|GetOrthoWidth (Variables|/Game/Blueprints/BP_Player.BP_Player_C|GetCamera (Variables|Default|GetPlayer)))))

(event EventBeginPlay
  ;[0.8047 0 1] Alles wichtige holen
  (bind _asbp_player (Utilities|Casting|CastToBP_Player (Game|Player|GetPlayerPawn 0)))
  (bind _output_get (Variables|Default|SetPlayer _asbp_player))
  (Variables|Default|SetLag (Variables|/Game/Blueprints/BP_Player.BP_Player_C|GetInterp%20Speed _output_get))
  (bind _asgm_plattformer (Utilities|Casting|CastToGM_Plattformer (Game|GetGameMode)))
  (Variables|Default|SetGameMode _asgm_plattformer)
  (CallFunction|GetCamerawith))

(event Collision|EventActorBeginOverlap
  (params (OtherActor :type Actor%20Object%20Reference))
  ;[0.2188 0 1] Player nochmal finden
  (if (== OtherActor (Game|Player|GetPlayerPawn 0))
    (bind _asbp_player (Utilities|Casting|CastToBP_Player (Game|Player|GetPlayerPawn 0)))
    (Variables|Default|SetPlayer _asbp_player)
    ;[0 1 0.1094] Fade Out
    (CameraFades|StartCameraFade :self (Game|GetPlayerCameraManager 0) :ToAlpha 1.0 :Duration 0.2 :bHoldWhenFinished true)
    ;[0 0.8359 1] Input Disablen und kurz auf den Fade warten
    (Utilities|FlowControl|Delay 0.2)
    (Input|DisableInput (Variables|Default|GetPlayer) (Game|GetPlayerController 0))
    ;[0.7109 0 1] Spline Change
    (Variables|/Game/Blueprints/BP_Player.BP_Player_C|SetInterp%20Speed (Variables|Default|GetPlayer) 0.0)
    (Default|ActiveSplineRef (Variables|Default|GetGameMode) (Variables|Default|GetCameraSpline%20))
    (Utilities|FlowControl|Delay 0.2)
    ;[0.6641 0 1] Aktiviere Input
    (Input|EnableInput (Variables|Default|GetPlayer) (Game|GetPlayerController 0))
    ;[0 0.7891 1] Fade in
    (CameraFades|StartCameraFade :self (Game|GetPlayerCameraManager 0) :FromAlpha 1.0 :Duration 0.5 :bHoldWhenFinished true)
    (Variables|/Game/Blueprints/BP_Player.BP_Player_C|SetInterp%20Speed (Variables|Default|GetPlayer) (Variables|Default|GetLag))
    (CallFunction|GetCamerawith)
    (CallFunction|CamerawithChange)))

(fn ConstructionScript)