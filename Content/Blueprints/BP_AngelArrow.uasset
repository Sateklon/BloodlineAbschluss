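; BP_AngelArrow is a projectile actor that damages only the player and destroys itself after a short lifetime.
; An external call sets its damage, and BeginPlay caches the player pawn as BP_Player.
; On sphere overlap it stops the projectile movement, applies BP_DamageNormal damage if it hit the player, and destroys itself.
; Overlapping any other actor sets a HitGround flag that blocks damage, then also destroys the arrow.
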(event OnComponentBeginOverlap(Sphere)
  (params (OverlappedComponent :type Primitive%20Component%20Object%20Reference) (OtherActor :type Actor%20Object%20Reference) (OtherComp :type Primitive%20Component%20Object%20Reference) (OtherBodyIndex :type Integer) (bFromSweep :type Boolean) (SweepResult :type Hit%20Result%20Structure%20%28by%20ref%29))
  ;[0 1 0.08594] Pfeilgedöns
  (if (== OtherActor (Variables|Default|GetPlayer))
    ;;[0.6172 1 0] Player getroffen
    (Game|Components|ProjectileMovement|StopSimulating (Variables|Default|GetProjectileMovement) SweepResult)
    ;;[0.6406 0 1] Make Damage
    (if (not (Variables|Default|GetHitGround))
      (Game|Damage|ApplyDamage OtherActor (Variables|Default|GetDamage) 0 self "/Game/Blueprints/Data/BP_DamageNormal.BP_DamageNormal_C")
      (Actor|DestroyActor))
    (else
      ;;[0.8516 0 1] Im Boden Stecken geblieben
      (Game|Components|ProjectileMovement|StopSimulating (Variables|Default|GetProjectileMovement) SweepResult)
      (Variables|Default|SetHitGround true)
      (Actor|DestroyActor))))

(event Custom|Set%20Arrow%20Damage
  (params (Damage :type Float%20%28double-precision%29))
  ;[0 0.7656 1] Get the Projectile Damage
  (Variables|Default|SetDamage Damage))

(event EventBeginPlay
  ;[0 1 0.2734] Lifecycle
  (bind _asbp_player (Utilities|Casting|CastToBP_Player (Game|Player|GetPlayerPawn 0)))
  (Variables|Default|SetPlayer _asbp_player)
  (Utilities|FlowControl|Delay 4.0)
  (Actor|DestroyActor))

(fn ConstructionScript)